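; Player controller for the shooting game that passes the player's name to their player state and stores team assignment.
; On possess, it calls ReqClientProcess, which reads the name from ShootingGameInstance and forwards it through ServerNewPlayerName to BP_ShootingPlayerState.
; The event names suggest a client-then-server round trip for the name.
; Separate request events, added for team splitting, set the team number and the number within the team.
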(event `self.ReceivePossess`
  (params (PossessedPawn :type "Pawn Object Reference"))
  (`self.Req Client Process`))

(event `Req Client Process`
  (bind _asshooting_game_instance (cast `/Game/ShootingGame/GameMode/ShootingGameInstance` (`GameplayStatics.GetGameInstance`)))
  (`self.Server New Player Name` (`/Game/ShootingGame/GameMode/ShootingGameInstance.Name` _asshooting_game_instance)))

(event `Server New Player Name`
  (params (`New Name` :type String))
  (bind _asbp_shooting_player_state (cast `/Game/ShootingGame/GameMode/BP_ShootingPlayerState` (`self.PlayerState`)))
  (`/Game/ShootingGame/GameMode/BP_ShootingPlayerState.Set Name` _asbp_shooting_player_state `New Name`))

(event `ReqSetTeamNumber`
  (params (TeamNumber :type Integer))
  ;[1 1 1] 팀 나누기할때 추가된 노드입니다.
  (set `self.TeamNumber` TeamNumber))

(event `ReqSetNumberInTeam`
  (params (NumberInTeam :type Integer))
  ;[1 1 1] 팀 나누기할때 추가된 노드입니다.
  (set `self.NumberInTeam` NumberInTeam))

(fn `UserConstructionScript`)