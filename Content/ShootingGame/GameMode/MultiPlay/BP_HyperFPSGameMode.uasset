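; Multiplayer FPS game mode that runs a two-team match from player join to final kill tally.
; Joining players are balanced into Team A or B, capped at half the lobby count.
; A BeginPlay delay sets Ready, then Tick steps through GameState phases with DoOnce gates: spawning at team-tagged points, starting, pausing and totalling kills.
; Late joiners spawn immediately during play, and leavers' kills are added to their team's total.
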(event `self.ReceiveBeginPlay`
  ;[1 1 1] Begin Event -> Game Init
  (`self.Init Game State`)
  (bind _asshooting_game_instance (cast `/Game/ShootingGame/GameMode/ShootingGameInstance` (`GameplayStatics.GetGameInstance`)))
  (bind _output_get (set `self.Game Instance` _asshooting_game_instance))
  (set `self.NumberOfPlayersInOneTeam` (`KismetMathLibrary.FCeil` (/ (`KismetMathLibrary.Conv_IntToDouble` (`/Game/ShootingGame/GameMode/ShootingGameInstance.Player Count` _output_get)) 2.0))) ; 한팀에 최대 몇명 들어가는지 세팅
  (`KismetSystemLibrary.Delay` 25.0) ; 로딩 30초 기다림
  (if (`|EnumInequality` (`/Game/ShootingGame/GameMode/MultiPlay/BP_HyperGameState.Game State` (`self.Game State`)) "NewEnumerator1")
    (set `/Game/ShootingGame/GameMode/MultiPlay/BP_HyperGameState.Game State` "NewEnumerator0" (`self.Game State`))))

(event `self.K2_PostLogin`
  (params (NewPlayer :type "PlayerController Object Reference"))
  ;[1 1 1] On Post
  (`self.Check All Player Login`))

(event `self.HandleStartingNewPlayer`
  (params (NewPlayer :type "PlayerController Object Reference"))
  (bind _returnvalue (`KismetMathLibrary.RandomInteger` 1))
  (bind _game_state (`self.Game State`))
  ;[1 1 1] Player Team 배정
  (bind _asbp_hyper_fpsplayer_controller (cast `/Game/ShootingGame/GameMode/MultiPlay/BP_HyperFPSPlayerController` NewPlayer))
  (`/Game/ShootingGame/GameMode/MultiPlay/BP_HyperFPSPlayerController.Req Client Process` _asbp_hyper_fpsplayer_controller) ; 컨트롤러/스테이트에 이름 Set
  (set `self.Player Controller` _asbp_hyper_fpsplayer_controller)
  (switch `int` (`self.Any Team Full?`) ; 0 : 팀 모두 안참\n1 : A 팀 꽉참\n2 : B 팀 꽉참
    (:`0`
      (if (== (`self.A Team Count`) (`self.B Team Count`))
        (if (== _returnvalue 0)
          (set `self.A Team Count` (+ (`self.A Team Count`) 1))
          (`KismetArrayLibrary.Array_Add` (`self.PlayerList_ATeam`) (`self.Player Controller`))
          (else
            (set `self.B Team Count` (+ (`self.B Team Count`) 1))
            (`KismetArrayLibrary.Array_Add` (`self.PlayerList_BTeam`) (`self.Player Controller`))))
        (`/Game/ShootingGame/GameMode/MultiPlay/BP_HyperFPSPlayerController.ReqSetTeamNumber` (`self.Player Controller`) _returnvalue)
        (elif (> (`self.A Team Count`) (`self.B Team Count`))
          (set `self.B Team Count` (+ (`self.B Team Count`) 1) :!label _label)
          (`KismetArrayLibrary.Array_Add` (`self.PlayerList_BTeam`) (`self.Player Controller`))
          (`/Game/ShootingGame/GameMode/MultiPlay/BP_HyperFPSPlayerController.ReqSetTeamNumber` (`self.Player Controller`) 1)
          (else
            (set `self.A Team Count` (+ (`self.A Team Count`) 1) :!label _label_2)
            (`KismetArrayLibrary.Array_Add` (`self.PlayerList_ATeam`) (`self.Player Controller`))
            (`/Game/ShootingGame/GameMode/MultiPlay/BP_HyperFPSPlayerController.ReqSetTeamNumber` (`self.Player Controller`) 0)))))
    (:`1`
      (goto _label))
    (:`2`
      (goto _label_2)))
  (`KismetArrayLibrary.Array_Add` (`self.PlayerList`) (`self.Player Controller`)) ; 컨트롤러 배열에 저장
  (`self.Check Team Full`) ; 한 팀이라도 꽉 찬 상태인지 체크
  (`/Engine/EditorBlueprintResources/StandardMacros.IsValid` _game_state
    (:`Is Valid`
      (if (`|EnumEquality` (`/Game/ShootingGame/GameMode/MultiPlay/BP_HyperGameState.Game State` _game_state) "NewEnumerator1")
        (`self.Possess Player` (`self.Player Controller`))))))

(event `Possess Player`
  (params (`Player Controller` :type "/Game/ShootingGame/GameMode/MultiPlay/BP_HyperFPSPlayerController Object Reference"))
  ;[1 1 1] Game Ready
  (if (== (`/Game/ShootingGame/GameMode/MultiPlay/BP_HyperFPSPlayerController.TeamNumber` `Player Controller`) 0)
    (bind _outactors (`GameplayStatics.GetAllActorsWithTag` "TeamA")) ; Random Player Start( A Team)
    (bind _output_get (set `/Game/ShootingGame/GameMode/MultiPlay/BP_HyperFPSPlayerController.Team` "NewEnumerator0" `Player Controller`))
    (bind _returnvalue (`|SpawnActorFromClass` "/Game/ShootingGame/GameMode/BP_HyperCharacter.BP_HyperCharacter_C" (`self.GetTransform` (`|GetArrayItem` _outactors (`KismetMathLibrary.RandomInteger` 3))) "AdjustIfPossibleButAlwaysSpawn" "OverrideRootScale" null "NewEnumerator0" `Player Controller` null))
    (bind _asbp_shooting_player_state (cast `/Game/ShootingGame/GameMode/BP_ShootingPlayerState` (`Controller.PlayerState` `Player Controller`)))
    (set `/Game/ShootingGame/GameMode/BP_ShootingPlayerState.Team` _output_get _asbp_shooting_player_state)
    (`KismetSystemLibrary.PrintString` "A" false false (struct :`R` 1.0 :`A` 1.0) 15.0)
    (`Controller.Possess` `Player Controller` _returnvalue)
    (else
      (bind _outactors_2 (`GameplayStatics.GetAllActorsWithTag` "TeamB")) ; Random Player Start( B Team)
      (bind _output_get_2 (set `/Game/ShootingGame/GameMode/MultiPlay/BP_HyperFPSPlayerController.Team` "NewEnumerator1" `Player Controller`))
      (bind _returnvalue_2 (`|SpawnActorFromClass` "/Game/ShootingGame/GameMode/BP_HyperCharacter.BP_HyperCharacter_C" (`self.GetTransform` (`|GetArrayItem` _outactors_2 (`KismetMathLibrary.RandomInteger` 3))) "AdjustIfPossibleButAlwaysSpawn" "OverrideRootScale" null "NewEnumerator1" `Player Controller` null))
      (bind _asbp_shooting_player_state_2 (cast `/Game/ShootingGame/GameMode/BP_ShootingPlayerState` (`Controller.PlayerState` `Player Controller`)))
      (set `/Game/ShootingGame/GameMode/BP_ShootingPlayerState.Team` _output_get_2 _asbp_shooting_player_state_2)
      (`KismetSystemLibrary.PrintString` "B" false false (struct :`R` 1.0 :`A` 1.0) 15.0)
      (`Controller.Possess` `Player Controller` _returnvalue_2))))

(event `self.ReceiveTick`
  (params (DeltaSeconds :type "Float (single-precision)"))
  (bind _total_kill_a_team (`self.Total Kill A Team`))
  (bind _total_kill_b_team (`self.Total Kill B Team`))
  (bind _game_state (`self.Game State`))
  ;[1 1 1] Tick
  (`/Engine/EditorBlueprintResources/StandardMacros.IsValid` (`self.Game State`)
    (:`Is Valid`
      (switch `/Game/ShootingGame/Data/Enum_GameState` (`/Game/ShootingGame/GameMode/MultiPlay/BP_HyperGameState.Game State` (`self.Game State`))
        (:`NewEnumerator0`
          ;[1 1 1] Game Ready
          (`/Engine/EditorBlueprintResources/StandardMacros.DoOnce` false
            (:`Completed`
              (for _array_element (`self.PlayerList`)
                (`self.Possess Player` _array_element))
              (if (`|EnumInequality` (`/Game/ShootingGame/GameMode/MultiPlay/BP_HyperGameState.Game State` (`self.Game State`)) "NewEnumerator1")
                (set `/Game/ShootingGame/GameMode/MultiPlay/BP_HyperGameState.Game State` "NewEnumerator1" (`self.Game State`))))))
        (:`NewEnumerator1`
          ;[1 1 1] Game Start
          (`/Engine/EditorBlueprintResources/StandardMacros.DoOnce` false
            (:`Completed`
              (bind _asbp_hyper_game_state (cast `/Game/ShootingGame/GameMode/MultiPlay/BP_HyperGameState` (`GameplayStatics.GetGameState`)))
              (`/Game/ShootingGame/GameMode/MultiPlay/BP_HyperGameState.Game Start` _asbp_hyper_game_state))))
        (:`NewEnumerator2`
          ;[1 1 1] Game End
          (`/Engine/EditorBlueprintResources/StandardMacros.DoOnce` false
            (:`Completed`
              (`|ExecutionSequence`
                (:`then_0`
                  (for _array_element_2 (`self.PlayerList_ATeam`)
                    (`/Engine/EditorBlueprintResources/StandardMacros.IsValid` _array_element_2
                      (:`Is Valid`
                        (bind _asbp_shooting_player_state (cast `/Game/ShootingGame/GameMode/BP_ShootingPlayerState` (`Controller.PlayerState` _array_element_2)))
                        (set `self.Total Kill A Team` (+ (`/Game/ShootingGame/GameMode/BP_ShootingPlayerState.Kill` _asbp_shooting_player_state) (`self.Total Kill A Team`))) ; A Team Total Kill 계산
                      ))))
                (:`then_1`
                  (for _array_element_3 (`self.PlayerList_BTeam`)
                    (`/Engine/EditorBlueprintResources/StandardMacros.IsValid` _array_element_3
                      (:`Is Valid`
                        (bind _asbp_shooting_player_state_2 (cast `/Game/ShootingGame/GameMode/BP_ShootingPlayerState` (`Controller.PlayerState` _array_element_3)))
                        (set `self.Total Kill B Team` (+ (`/Game/ShootingGame/GameMode/BP_ShootingPlayerState.Kill` _asbp_shooting_player_state_2) (`self.Total Kill B Team`))) ; B Team Total Kill 계산
                      )))
                  (`/Game/ShootingGame/GameMode/MultiPlay/BP_HyperGameState.Result Kill` _game_state _total_kill_a_team _total_kill_b_team)
                  (`KismetSystemLibrary.PrintString` (`KismetStringLibrary.Concat_StrStr` "A Team Kill :  " (`KismetStringLibrary.Conv_IntToString` _total_kill_a_team) "B Team Kill :  " (`KismetStringLibrary.Conv_IntToString` _total_kill_b_team)) false false (struct :`R` 1.0 :`B` 0.297748 :`A` 1.0) 30.0)
                  (set `/Game/ShootingGame/GameMode/MultiPlay/BP_HyperGameState.Game State` "NewEnumerator5" _game_state))))))
        (:`NewEnumerator3`
          (`/Engine/EditorBlueprintResources/StandardMacros.DoOnce` false
            (:`Completed`
              (`GameplayStatics.SetGamePaused` true))))))))

(event `self.K2_OnLogout`
  (params (ExitingController :type "Controller Object Reference"))
  ;[1 1 1] Logout
  (bind _asbp_shooting_player_state (cast `/Game/ShootingGame/GameMode/BP_ShootingPlayerState` (`Controller.PlayerState` ExitingController)))
  (switch `/Game/ShootingGame/Data/Character_Team` (`/Game/ShootingGame/GameMode/BP_ShootingPlayerState.Team` _asbp_shooting_player_state)
    (:`NewEnumerator0`
      (set `self.Total Kill A Team` (+ (`/Game/ShootingGame/GameMode/BP_ShootingPlayerState.Kill` _asbp_shooting_player_state) (`self.Total Kill A Team`))))
    (:`NewEnumerator1`
      (set `self.Total Kill B Team` (+ (`/Game/ShootingGame/GameMode/BP_ShootingPlayerState.Kill` _asbp_shooting_player_state) (`self.Total Kill B Team`))))))

(fn `Check All Player Login`
  (`/Engine/EditorBlueprintResources/StandardMacros.IsValid` (`self.Game Instance`)
    (:`Is Valid`
      (bind _output_get (set `self.On Post Login Player` (+ (`self.On Post Login Player`) 1)))
      (set `/Game/ShootingGame/GameMode/MultiPlay/BP_HyperGameState.On Post Controller` _output_get (`self.Game State`))
      (if (== (`/Game/ShootingGame/GameMode/ShootingGameInstance.Player Count` (`self.Game Instance`)) (`self.On Post Login Player`))
        (if (`|EnumInequality` (`/Game/ShootingGame/GameMode/MultiPlay/BP_HyperGameState.Game State` (`self.Game State`)) "NewEnumerator1")
          _)))
    (:`Is Not Valid`
      (`KismetSystemLibrary.K2_SetTimer` null "Check All Player Login" 0.1))))

(fn `Check Spawn Armor`
  (params (`Own Spawner` :type "/Game/ShootingGame/Blueprint/Armor/Armor_Spawner Object Reference"))
  (`/Game/ShootingGame/Blueprint/Armor/Armor_Spawner.Random Spawn` `Own Spawner`))

(fn `Check Spawn Item`
  (params (`Own Spawner` :type "/Game/ShootingGame/Blueprint/Item/BP_SpawnArea Object Reference"))
  (`/Game/ShootingGame/Blueprint/Item/BP_SpawnArea.Random Spawn` `Own Spawner`))

(fn `Check Spawn Skill`
  (params (`Own Spawner` :type "/Game/ShootingGame/Blueprint/Skill/Skill_Spawner Object Reference")))

(fn `Check Team Full`
  (bind _returnvalue (== (`self.B Team Count`) (`self.NumberOfPlayersInOneTeam`)))
  (if (== (`self.A Team Count`) (`self.NumberOfPlayersInOneTeam`))
    (if (not _returnvalue)
      (set `self.Any Team Full?` 1) ; A 꽉참
    )
    (elif _returnvalue
      (set `self.Any Team Full?` 2) ; B 꽉참
      (else
        (set `self.Any Team Full?` 0) ; 둘 다 꽉 안참\n-> 디폴트가 0 이므로 변경 x
      ))))

(fn `Init Game State`
  (bind _asbp_hyper_game_state (cast `/Game/ShootingGame/GameMode/MultiPlay/BP_HyperGameState` (`GameplayStatics.GetGameState`))
    (:`then`
      (set `self.Game State` _asbp_hyper_game_state))
    (:`CastFailed`
      (`KismetSystemLibrary.K2_SetTimer` null "Init Game State" 0.1))))

(fn `UserConstructionScript`)