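; Multiplayer player controller for HyperFPS that handles player naming, team slot assignment and text chat.
; On possession it reads the name from the game instance and passes it through a server-named event to the player state.
; All and team chat events loop over the game mode's PlayerList, filtering by Team for team chat.
; Each recipient controller forwards the message to the chat widget in its HUD, cached at BeginPlay.
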(event `self.ReceivePossess`
  (params (PossessedPawn :type "Pawn Object Reference"))
  (`self.Req Client Process`))

(event `Req Client Process`
  (bind _asshooting_game_instance (cast `/Game/ShootingGame/GameMode/ShootingGameInstance` (`GameplayStatics.GetGameInstance`)))
  (`self.Server New Player Name` (`/Game/ShootingGame/GameMode/ShootingGameInstance.Name` _asshooting_game_instance)))

(event `Server New Player Name`
  (params (`New Name` :type String))
  (bind _asbp_shooting_player_state (cast `/Game/ShootingGame/GameMode/BP_ShootingPlayerState` (`self.PlayerState`)))
  (bind _output_get (set `self.Name` `New Name`))
  (`KismetSystemLibrary.PrintString` _output_get false false (struct :`G` 0.088777 :`B` 1.0 :`A` 1.0) 20.0)
  (`/Game/ShootingGame/GameMode/BP_ShootingPlayerState.Set Name` _asbp_shooting_player_state `New Name`))

(event `ReqSetTeamNumber`
  (params (TeamNumber :type Integer))
  ;[1 1 1] 팀 나누기할때 추가된 노드입니다.
  (set `self.TeamNumber` TeamNumber))

(event `ReqSetNumberInTeam`
  (params (NumberInTeam :type Integer))
  ;[1 1 1] 팀 나누기할때 추가된 노드입니다.
  (set `self.NumberInTeam` NumberInTeam))

(event `SendChatAllMessage`
  (params (`Send Message` :type String))
  (bind _asbp_hyper_fpsgame_mode (cast `/Game/ShootingGame/GameMode/MultiPlay/BP_HyperFPSGameMode` (`GameplayStatics.GetGameMode`)))
  (for _array_element (`/Game/ShootingGame/GameMode/MultiPlay/BP_HyperFPSGameMode.PlayerList` _asbp_hyper_fpsgame_mode)
    (`self.Update Chat Log` _array_element (`self.Name`) `Send Message` "All") ; 이름하고 메세지 소유 클라(Controller)로 넘김
  ))

(event `self.ReceiveBeginPlay`
  (bind _asbp_shooting_hud (cast `/Game/ShootingGame/GameMode/BP_ShootingHUD` (`self.GetHUD` (`GameplayStatics.GetPlayerController` 0))))
  (set `self.HUD` _asbp_shooting_hud))

(event `SendChatTeamMessage`
  (params (`Send Message` :type String) (`Send Player Team` :type "/Game/ShootingGame/Data/Character_Team Enum" :default "NewEnumerator0"))
  (bind _asbp_hyper_fpsgame_mode (cast `/Game/ShootingGame/GameMode/MultiPlay/BP_HyperFPSGameMode` (`GameplayStatics.GetGameMode`)))
  (for _array_element (`/Game/ShootingGame/GameMode/MultiPlay/BP_HyperFPSGameMode.PlayerList` _asbp_hyper_fpsgame_mode)
    (if (`|EnumEquality` (`/Game/ShootingGame/GameMode/MultiPlay/BP_HyperFPSPlayerController.Team` _array_element) `Send Player Team`)
      (`self.Update Chat Log` _array_element (`self.Name`) `Send Message` "Team") ; 이름하고 메세지 소유 클라(Controller)로 넘김
    )))

(event `Update Chat Log`
  (params (`Player Name` :type String) (Message :type String) (`Chat Type` :type String))
  (`/Game/ShootingGame/Widget/Chatting_Widget.Update Chat Log` (`/Game/ShootingGame/Widget/ShootingHUDWidget.Chatting_Widget` (`/Game/ShootingGame/GameMode/BP_ShootingHUD.Hud Widget` (`self.HUD`))) (make `/Game/ShootingGame/Data/ST_Chat` `Player Name` Message `Chat Type`)))

(fn `UserConstructionScript`)