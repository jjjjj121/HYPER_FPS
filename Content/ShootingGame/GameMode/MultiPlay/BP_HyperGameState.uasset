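; Multiplayer game state for the shooting game that tracks match phase, play time and two-team kill totals.
; BeginPlay takes the time limit and player count from the game instance.
; Tick switches on GameState to show loading, end and result widgets, and drives a server-only gated timer that formats clock text and ends the match at the limit.
; An OnRep on the posted-controller value broadcasts the player count through a dispatcher.
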(event `self.ReceiveBeginPlay`
  (bind _asbp_hyper_fpsgame_mode (cast `/Game/ShootingGame/GameMode/MultiPlay/BP_HyperFPSGameMode` (`GameplayStatics.GetGameMode`)))
  (set `self.Game Mode` _asbp_hyper_fpsgame_mode)
  (bind _asshooting_game_instance (cast `/Game/ShootingGame/GameMode/ShootingGameInstance` (`GameplayStatics.GetGameInstance`)))
  (set `self.End Play Time` (`/Game/ShootingGame/GameMode/ShootingGameInstance.Play Time` _asshooting_game_instance))
  (set `self.Max Player Count` (`/Game/ShootingGame/GameMode/ShootingGameInstance.Player Count` _asshooting_game_instance)))

(event `Game Start`
  (bind _returnvalue (`KismetMathLibrary.FFloor` (`self.Play Time Second`)))
  (goto _label :!via `Open`))

(event `Game End`
  (bind _returnvalue (`KismetMathLibrary.FFloor` (`self.Play Time Second`)))
  (goto _label :!via `Close`))

(event `self.ReceiveTick`
  (params (DeltaSeconds :type "Float (single-precision)"))
  (bind _returnvalue (`KismetMathLibrary.FFloor` (`self.Play Time Second`)))
  (switch `/Game/ShootingGame/Data/Enum_GameState` (`self.Game State`)
    (:`NewEnumerator1`
      (`|ExecutionSequence`
        (:`then_0`
          (`/Engine/EditorBlueprintResources/StandardMacros.DoOnce` false ; Loding
            (:`Completed`
              (`Widget.RemoveFromParent` (`self.Loading Widget`)))))
        (:`then_1`
          (`/Engine/EditorBlueprintResources/ActorMacros.Switch Has Authority` ; 서버에서만 시간관리
            (:`Authority`
              (`/Engine/EditorBlueprintResources/StandardMacros.Gate` true :!label _label
                (:`Exit`
                  (if (>= (`self.Play Time Minutes`) (`self.End Play Time`))
                    (`self.Game End`)
                    (set `self.Game State` "NewEnumerator2")
                    (elif (>= (`self.Play Time Second`) 60.0)
                      (set `self.Play Time Second` 0.0)
                      (set `self.Play Time Minutes` (+ (`self.Play Time Minutes`) 1))
                      (else
                        (set `self.Play Time Second` (+ DeltaSeconds (`self.Play Time Second`)))
                        (if (< _returnvalue 10)
                          (set `self.Time Text` (`|FormatText` "{Minutes} : 0{Second}" (`self.Play Time Minutes`) _returnvalue))
                          (else
                            (set `self.Time Text` (`|FormatText` "{Minutes} : {Second}" (`self.Play Time Minutes`) _returnvalue))))))))))))))
    (:`NewEnumerator4`
      (`/Engine/EditorBlueprintResources/StandardMacros.DoOnce` false ; Loding
        (:`Completed`
          (bind _returnvalue_2 (`|CreateWidget` "/Game/ShootingGame/Widget/LoadingWidget.LoadingWidget_C" null (`self.Max Player Count`) (`self.On Post Controller`)))
          (bind _output_get (set `self.Loading Widget` _returnvalue_2))
          (`UserWidget.AddToViewport` _output_get 0))))
    (:`NewEnumerator5`
      (`/Engine/EditorBlueprintResources/StandardMacros.DoOnce` false
        (:`Completed`
          (`WidgetLayoutLibrary.RemoveAllWidgets`)
          (bind _returnvalue_3 (`|CreateWidget` "/Game/ShootingGame/Widget/End_Widget.End_Widget_C"))
          (`UserWidget.AddToViewport` _returnvalue_3 0)
          (`KismetSystemLibrary.Delay` 4.0)
          (`WidgetLayoutLibrary.RemoveAllWidgets`)
          (bind _returnvalue_4 (`|CreateWidget` "/Game/ShootingGame/Widget/Result/GameResultWidget.GameResultWidget_C" null (`self.Total Kill A Team`) (`self.Total Kill B Team`)))
          (`UserWidget.AddToViewport` _returnvalue_4 0))))))

(event `Result Kill`
  (params (`Total Kill A Team` :type Integer) (`Total Kill B Team` :type Integer))
  (set `self.Total Kill A Team` `Total Kill A Team`)
  (set `self.Total Kill B Team` `Total Kill B Team`))

(fn `OnRep_On Post Controller`
  (`self.EventDispatcher_PlayerCount` (`self.On Post Controller`))
  (`KismetSystemLibrary.PrintString` "호출!!!!!!!!!!!!" false false (struct :`R` 0.86074 :`B` 1.0 :`A` 1.0) 30.0))

(fn `UserConstructionScript`)