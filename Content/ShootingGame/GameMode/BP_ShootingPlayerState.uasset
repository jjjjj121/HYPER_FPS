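; Player state for the shooting game, holding each player's armor, base and buff HP, team, name, kills and deaths.
; Damage cascades from armor through buff HP to base HP, whose sum drives the death check.
; RepNotifies fire event dispatchers, refresh the HUD player list, and update shield durability and body skin by team and armor tier.
; BeginPlay binds to the shooting HUD and retries on a timer until the pawn is valid.
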(event `self.ReceiveBeginPlay`
  (`self.Init Bind`)
  (`KismetSystemLibrary.PrintString` (`KismetStringLibrary.Concat_StrStr` "Create  " (`KismetSystemLibrary.GetDisplayName` self) "  Pawn -" (`KismetSystemLibrary.GetDisplayName` (`self.PawnPrivate`))) false false (struct :`G` 0.66 :`B` 1.0 :`A` 1.0) 30.0)
  (`self.Init My Pawn`))

(event `self.ReceiveTick`
  (params (DeltaSeconds :type "Float (single-precision)")))

(event `Server Set Armor`
  (params (Armor :type "Float (double-precision)"))
  (set `self.Armor` Armor))

(fn `Add Armor`
  (params (B :type "Float (double-precision)"))
  (set `self.Armor` (`KismetMathLibrary.FClamp` (+ (`self.Armor`) B) 0.0 (`self.Max Armor`))))

(fn `Add Damage`
  (params (Damage :type "Float (double-precision)") (`Hyper FPS Character` :type "/Game/ShootingGame/GameMode/BP_HyperCharacter Object Reference"))
  (bind _returnvalue (- (`self.Armor`) Damage))
  (bind _returnvalue_2 (+ (`self.Buff HP`) _returnvalue))
  (if (> _returnvalue 0.0)
    (set `self.Armor` (`KismetMathLibrary.FClamp` (- (`self.Armor`) (`local.Damage`)) 0.0 200.0))
    (else
      (set `self.Armor` 0.0)
      (if (> (`self.Buff HP`) 0.0)
        (if (> _returnvalue_2 0.0)
          (set `self.Buff HP` (`KismetMathLibrary.FClamp` _returnvalue_2 0.0 50.0))
          (else
            (set `self.Buff HP` 0.0)
            (set `self.Base HP` (`KismetMathLibrary.FClamp` (+ (`self.Base HP`) _returnvalue_2) 0.0 100.0))))
        (else
          (set `self.Base HP` (`KismetMathLibrary.FClamp` (+ (`self.Base HP`) _returnvalue) 0.0 100.0)))))))

(fn `Add Death`
  (set `self.Death` (+ (`self.Death`) 1)))

(fn `Add Heal`
  (params (B :type "Float (double-precision)"))
  (set `self.Base HP` (`KismetMathLibrary.FClamp` (+ (`self.Base HP`) B) 0.0 100.0)))

(fn `Add Kill`
  (set `self.Kill` (+ (`self.Kill`) 1)))

(fn `Change Skin`
  (bind _private_character (`self.Private Character`))
  (bind _mesh (`Character.Mesh` (`self.Private Character`)))
  (bind _mesh_2 (`Character.Mesh` (`self.Private Character`)))
  (`/Engine/EditorBlueprintResources/StandardMacros.IsValid` _private_character
    (:`Is Valid`
      (switch `/Game/ShootingGame/Data/Character_Team` (`/Game/ShootingGame/GameMode/BP_HyperCharacter.Team` _private_character)
        (:`NewEnumerator0`
          (`self.Check Armor Type`
            (:`Red`
              (`PrimitiveComponent.SetMaterialByName` _mesh_2 "Base" "/Game/ShootingGame/Met/Barrier_Skin_Red.Barrier_Skin_Red"))
            (:`Purple`
              (`PrimitiveComponent.SetMaterialByName` _mesh_2 "Base" "/Game/ShootingGame/Met/Barrier_Skin_Purple.Barrier_Skin_Purple"))
            (:`Blue`
              (`PrimitiveComponent.SetMaterialByName` _mesh_2 "Base" "/Game/ShootingGame/Met/Barrier_Skin_Blue.Barrier_Skin_Blue"))
            (:`Green`
              (`PrimitiveComponent.SetMaterialByName` _mesh_2 "Base" "/Game/ShootingGame/Met/Barrier_Skin_Green.Barrier_Skin_Green"))
            (:`False`
              (`PrimitiveComponent.SetMaterialByName` _mesh_2 "Base" "/Game/ShootingGame/Met/Barrier_Skin_Original.Barrier_Skin_Original"))))
        (:`NewEnumerator1`
          (`self.Check Armor Type`
            (:`Red`
              (`PrimitiveComponent.SetMaterialByName` _mesh "Base" "/Game/ShootingGame/Met/Barrier_Skin_Red_B.Barrier_Skin_Red_B"))
            (:`Purple`
              (`PrimitiveComponent.SetMaterialByName` _mesh "Base" "/Game/ShootingGame/Met/Barrier_Skin_Purple_B.Barrier_Skin_Purple_B"))
            (:`Blue`
              (`PrimitiveComponent.SetMaterialByName` _mesh "Base" "/Game/ShootingGame/Met/Barrier_Skin_Blue_B.Barrier_Skin_Blue_B"))
            (:`Green`
              (`PrimitiveComponent.SetMaterialByName` _mesh "Base" "/Game/ShootingGame/Met/Barrier_Skin_Green_B.Barrier_Skin_Green_B"))
            (:`False`
              (`PrimitiveComponent.SetMaterialByName` _mesh "Base" "/Game/ShootingGame/Met/Barrier_Skin_Original_B.Barrier_Skin_Original_B"))))))))

(fn `Drop Player Armor`
  (params (`Own Character` :type "/Game/ShootingGame/GameMode/BP_HyperCharacter Object Reference"))
  (bind _own_character (`local.Own Character`))
  (`self.Check Armor Type`
    (:`Red`
      (`|SpawnActorFromClass` "/Game/ShootingGame/Blueprint/Armor/Armor_Original.Armor_Original_C" (`KismetMathLibrary.MakeTransform` (+ (`self.K2_GetActorLocation` _own_character) (* (`self.GetActorForwardVector` _own_character) 100.0))) "Undefined" "OverrideRootScale" null 200.0 null 200.0 null null)
      (`KismetSystemLibrary.PrintString` "Hello" false false))))

(fn `Init Bind`
  (bind _asbp_shooting_hud (cast `/Game/ShootingGame/GameMode/BP_ShootingHUD` (`PlayerController.GetHUD` (`GameplayStatics.GetPlayerController` 0)))
    (:`then`
      (bind _output_get (set `self.Shooting HUD` _asbp_shooting_hud))
      (`/Game/ShootingGame/GameMode/BP_ShootingHUD.Bind Player State` _output_get self)
      (`KismetSystemLibrary.PrintString` (`|GetEnumeratorNameAsString` (`self.Team`)) false false (struct :`R` 1.0 :`G` 0.724876 :`A` 1.0) 60.0))
    (:`CastFailed`
      (`KismetSystemLibrary.PrintString` "BP_LobyHUD Cast Fail!" false false (struct :`R` 1.0 :`G` 0.030547 :`A` 1.0) 60.0))))

(fn `Init My Pawn`
  (`/Engine/EditorBlueprintResources/StandardMacros.IsValid` (`self.PawnPrivate`)
    (:`Is Valid`
      (bind _asbp_hyper_character (cast `/Game/ShootingGame/GameMode/BP_HyperCharacter` (`self.PawnPrivate`)))
      (set `self.Private Character` _asbp_hyper_character)
      (`self.Change Skin`))
    (:`Is Not Valid`
      (`KismetSystemLibrary.K2_SetTimer` null "Init My Pawn" 0.1))))

(fn `Init Tag`
  (switch `/Game/ShootingGame/Data/Character_Team` (`self.Team`)
    (:`NewEnumerator0`
      (`KismetArrayLibrary.Array_Add` (`self.Tags`) "TeamA")
      (`KismetSystemLibrary.PrintString` "Tag A" false false))
    (:`NewEnumerator1`
      (`KismetArrayLibrary.Array_Add` (`self.Tags`) "TeamB")
      (`KismetSystemLibrary.PrintString` "Tag B" false false))))

(fn `Is Death`
  (returns (`Is Die` :type Boolean))
  (if (<= (`self.Result HP`) 0.0)
    (return true)
    (else
      (return false))))

(fn `OnRep_Armor`
  (`self.EventDispatcher_Armor` (`self.Armor`) (`self.Max Armor`))
  (`self.Change Skin`)
  (`/Inventory3/InventorySystem/ActorComponent/ItemTemplatePickupComponent.Update Shield Durability` (`/Game/ShootingGame/GameMode/BP_HyperCharacter.TemplatePickupComponent` (`self.Private Character`)) (`KismetMathLibrary.FTrunc` (`self.Armor`))))

(fn `OnRep_Base HP`
  (set `self.Result HP` (+ (`self.Buff HP`) (`self.Base HP`))))

(fn `OnRep_Buff HP`
  (set `self.Result HP` (+ (`self.Buff HP`) (`self.Base HP`))))

(fn `OnRep_Death`
  (`self.EventDispatcher_Death` (`self.Death`)))

(fn `OnRep_Kill`
  (`self.EventDispatcher_Kill` (`self.Kill`)))

(fn `OnRep_Name`
  (`self.EventDispatcher_Name` (`self.Name`)))

(fn `OnRep_Result HP`
  (`KismetSystemLibrary.PrintString` "!@#!@#$!$!#!@#" false false (struct :`R` 0.0079 :`B` 1.0 :`A` 1.0) 10.0)
  (`self.EventDispatcher_HP` (`self.Base HP`) (`self.Buff HP`) 100.0 50.0))

(fn `OnRep_Team`
  (`/Game/ShootingGame/GameMode/BP_ShootingHUD.Update Player List` (`self.Shooting HUD`)))

(fn `Set Name`
  (params (Name :type String))
  (set `self.Name` Name))

(fn `UserConstructionScript`)