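; BP_ShootingHUD is the shooting game's HUD, creating the crosshair, hidden sniper scope and main HUD widgets at BeginPlay.
; It caches the owning character, sets game-only input and binds to the local PlayerState's HP and armor dispatchers, retrying by timer until that state exists.
; Update functions forward ammo, health, armor, weapon and item-guide data to the main widget.
; Name, kill and death events from bound PlayerStates refresh the team player list.
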(event `self.ReceiveBeginPlay`
  (bind _returnvalue (`GameplayStatics.GetPlayerController` 0))
  (`self.Init Widget`)
  (`self.Bind My Player State`)
  (`self.Init Pawn`)
  (`WidgetBlueprintLibrary.SetInputMode_GameOnly` _returnvalue)
  (set `PlayerController.bShowMouseCursor` false _returnvalue))

(fn `Bind My Player State`
  (bind _asbp_shooting_player_state (cast `/Game/ShootingGame/GameMode/BP_ShootingPlayerState` (`Controller.PlayerState` (`GameplayStatics.GetPlayerController` 0))) ; 시작하자마자 생성되는데, 생성되기 전에 캐스트로 접근하면 \ncast failed가 되므로 생성되서 캐스트 할 때 까지 재귀함수 돌리기
    (:`then`
      (set `self.Team` (`/Game/ShootingGame/GameMode/BP_ShootingPlayerState.Team` _asbp_shooting_player_state))
      (add `/Game/ShootingGame/GameMode/BP_ShootingPlayerState.EventDispatcher_HP` _asbp_shooting_player_state (`|CreateDelegate` :!event `Update HP`))
      (add `/Game/ShootingGame/GameMode/BP_ShootingPlayerState.EventDispatcher_Armor` _asbp_shooting_player_state (`|CreateDelegate` :!event `Update Armor`)))
    (:`CastFailed`
      (`KismetSystemLibrary.K2_SetTimer` null "Bind My Player State" 0.1))))

(fn `Bind Player State`
  (params (`Player State` :type "/Game/ShootingGame/GameMode/BP_ShootingPlayerState Object Reference"))
  (add `/Game/ShootingGame/GameMode/BP_ShootingPlayerState.EventDispatcher_Name` `Player State` (`|CreateDelegate` :!event `Event_ Change Name`))
  (add `/Game/ShootingGame/GameMode/BP_ShootingPlayerState.EventDispatcher_Kill` `Player State` (`|CreateDelegate` :!event `Event Kill`))
  (add `/Game/ShootingGame/GameMode/BP_ShootingPlayerState.EventDispatcher_Death` `Player State` (`|CreateDelegate` :!event `Event Death`))
  (`self.Update Player List`))

(fn `Event Death`
  (params (Death :type Integer))
  (`self.Update Player List`))

(fn `Event Kill`
  (params (kill :type Integer))
  (`self.Update Player List`))

(fn `Event_ Change Name`
  (params (Name :type String))
  (`self.Update Player List`))

(fn `Init Pawn`
  (bind _asbp_hyper_character (cast `/Game/ShootingGame/GameMode/BP_HyperCharacter` (`self.GetOwningPawn`)))
  (set `self.HyperCharacter` _asbp_hyper_character))

(fn `Init Widget`
  (bind _returnvalue (`|CreateWidget` "/Game/ShootingGame/Widget/Aim.Aim_C"))
  (set `self.Aim` _returnvalue)
  (bind _returnvalue_2 (`|CreateWidget` "/Game/ShootingGame/Widget/Sniper_Aim_Widget.Sniper_Aim_Widget_C"))
  (bind _output_get (set `self.Sniper Aim` _returnvalue_2))
  (`Widget.SetVisibility` _output_get "Collapsed")
  (bind _returnvalue_3 (`|CreateWidget` "/Game/ShootingGame/Widget/ShootingHUDWidget.ShootingHUDWidget_C"))
  (set `self.Hud Widget` _returnvalue_3)
  (`UserWidget.AddToViewport` _returnvalue_3 0)
  (`UserWidget.AddToViewport` _returnvalue 0)
  (`UserWidget.AddToViewport` _output_get 0))

(fn `Set Visibility Guide F`
  (params (InVisibility :type "ESlateVisibility Enum" :default "Visible"))
  (`/Game/ShootingGame/Widget/ShootingHUDWidget.SetVisibilityGuideInfo` (`self.Hud Widget`) InVisibility))

(fn `Update Armor`
  (params (CurArmor :type "Float (double-precision)") (MaxArmor :type "Float (double-precision)"))
  (`/Game/ShootingGame/Widget/ShootingHUDWidget.SetArmor` (`self.Hud Widget`) CurArmor MaxArmor))

(fn `Update Guide Info`
  (params (`World Location` :type "Vector Structure") (`Item Index` :type Integer) (`Hit Actor` :type "Actor Object Reference"))
  (`/Game/ShootingGame/Widget/ShootingHUDWidget.SetInformationWidget` (`self.Hud Widget`) `World Location` `Item Index` `Hit Actor`))

(fn `Update HP`
  (params (`Base HP` :type "Float (double-precision)") (`Buff HP` :type "Float (double-precision)") (`Base Max HP` :type "Float (double-precision)") (`Buff Max HP` :type "Float (double-precision)"))
  (`/Game/ShootingGame/Widget/ShootingHUDWidget.SetHP` (`self.Hud Widget`) `Base HP` `Buff HP` `Base Max HP` `Buff Max HP`))

(fn `Update Player List`
  (bind _hud_widget (`self.Hud Widget`))
  (`/Engine/EditorBlueprintResources/StandardMacros.IsValid` _hud_widget
    (:`Is Valid`
      (`/Game/ShootingGame/Widget/ShootingHUDWidget.Update Player List Team` _hud_widget))
    (:`Is Not Valid`
      (`KismetSystemLibrary.K2_SetTimer` null "Update Player List" 0.1))))

(fn `Update Weapon Widget`
  (params (`Item Index` :type Integer))
  (`/Game/ShootingGame/Widget/ShootingHUDWidget.Update Weapon` (`self.Hud Widget`) `Item Index`))

(fn `UpdateAmmo`
  (params (Ammo :type Integer))
  (`/Game/ShootingGame/Widget/ShootingHUDWidget.Set Ammo` (`self.Hud Widget`) Ammo))

(fn `UpdateMag`
  (params (Mag :type Integer))
  (`/Game/ShootingGame/Widget/ShootingHUDWidget.Set Mag` (`self.Hud Widget`) Mag))

(fn `UserConstructionScript`)