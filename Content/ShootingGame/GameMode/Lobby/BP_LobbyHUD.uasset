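; Lobby HUD that creates the lobby widget on BeginPlay, adds it to the viewport, and switches to UI-only input with a visible cursor.
; BindPlayerState hooks a player state's name-change dispatcher and immediately triggers a player list refresh on the widget.
; The refresh ignores the passed name and retries on a short timer until the widget is valid, covering binds that arrive before it exists.
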(event `self.ReceiveBeginPlay`
  (bind _returnvalue (`GameplayStatics.GetPlayerController` 0))
  (bind _returnvalue_2 (`|CreateWidget` "/Game/ShootingGame/Widget/Loby/LobbyHUDWidget.LobbyHUDWidget_C"))
  (bind _output_get (set `self.HUD Widget` _returnvalue_2))
  (`UserWidget.AddToViewport` _output_get 0)
  (`WidgetBlueprintLibrary.SetInputMode_UIOnlyEx` _returnvalue null)
  (set `PlayerController.bShowMouseCursor` true _returnvalue))

(fn `BindPlayerState`
  (params (PlayerState :type "/Game/ShootingGame/GameMode/Lobby/BP_LobbyPlayerState Object Reference"))
  (add `/Game/ShootingGame/GameMode/Lobby/BP_LobbyPlayerState.EventDispatcher_ChangeName` PlayerState (`|CreateDelegate` :!event `Event_ChangeName`))
  (`self.Event_ChangeName` ""))

(fn `Event_ChangeName`
  (params (NewName :type String))
  (`self.RF_ChangeName`))

(fn `RF_ChangeName`
  (`/Engine/EditorBlueprintResources/StandardMacros.IsValid` (`self.HUD Widget`)
    (:`Is Valid`
      (`/Game/ShootingGame/Widget/Loby/LobbyHUDWidget.UpdatePlayerList` (`self.HUD Widget`)))
    (:`Is Not Valid`
      (`KismetSystemLibrary.K2_SetTimer` null "RF_ChangeName" 0.1))))

(fn `UserConstructionScript`)