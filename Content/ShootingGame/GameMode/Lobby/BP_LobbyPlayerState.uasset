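; Lobby player state that holds a player's name and announces changes to it.
; On BeginPlay it gets the HUD of player controller 0, casts it to BP_LobbyHUD and passes itself in for binding.
; A setter writes Name, and its OnRep function fires the change-name event dispatcher with the new value so listeners can update.
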(event `self.ReceiveBeginPlay`
  (`self.InitBind`))

(fn `InitBind`
  (bind _asbp_lobby_hud (cast `/Game/ShootingGame/GameMode/Lobby/BP_LobbyHUD` (`PlayerController.GetHUD` (`GameplayStatics.GetPlayerController` 0)))
    (:`then`
      (`/Game/ShootingGame/GameMode/Lobby/BP_LobbyHUD.BindPlayerState` _asbp_lobby_hud self))
    (:`CastFailed`
      (`KismetSystemLibrary.PrintString` "BP_LobyHUD Cast Fail!" false false (struct :`R` 1.0 :`G` 0.030547 :`A` 1.0) 60.0))))

(fn `OnRep_Name`
  (`KismetSystemLibrary.PrintString` (`KismetStringLibrary.Concat_StrStr` "OnRepName :" (`self.Name`)) false false (struct :`G` 0.66 :`B` 1.0 :`A` 1.0) 60.0)
  (`self.EventDispatcher_ChangeName` (`self.Name`)) ; 플레이어가 이름이 바뀌면 호출
)

(fn `Set Name`
  (params (Name :type String))
  (set `self.Name` Name))

(fn `UserConstructionScript`)