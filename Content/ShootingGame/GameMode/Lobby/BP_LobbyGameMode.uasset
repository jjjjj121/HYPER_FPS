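; Lobby game mode for the shooting game that counts players as they log in.
; BeginPlay caches the ShootingGameInstance, and each PostLogin increments its PlayerCount, with no decrement in this graph.
; SetPlayerCount retries itself on a short timer until the cached instance is valid, covering logins that arrive before BeginPlay.
; Debug prints have screen and log output disabled, and InitInstance is an empty, unused stub.
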(event `self.ReceiveBeginPlay`
  (bind _asshooting_game_instance (cast `/Game/ShootingGame/GameMode/ShootingGameInstance` (`GameplayStatics.GetGameInstance`)))
  (set `self.Game Instance` _asshooting_game_instance))

(event `self.K2_PostLogin`
  (params (NewPlayer :type "PlayerController Object Reference"))
  (`parent.K2_PostLogin` NewPlayer)
  (`self.Set Player Count`)
  (`KismetSystemLibrary.PrintString` (`KismetStringLibrary.Concat_StrStr` "Login Player  :  " (`KismetSystemLibrary.GetDisplayName` NewPlayer)) false false (struct :`G` 0.66 :`B` 1.0 :`A` 1.0) 30.0))

(event `self.HandleStartingNewPlayer`
  (params (NewPlayer :type "PlayerController Object Reference"))
  (`parent.HandleStartingNewPlayer` NewPlayer)
  (`KismetSystemLibrary.PrintString` (`KismetStringLibrary.Concat_StrStr` "Ready Player  :  " (`KismetSystemLibrary.GetDisplayName` NewPlayer)) false false (struct :`R` 0.346722 :`G` 1.0 :`A` 1.0) 30.0))

(fn `Init Instance`)

(fn `Set Player Count`
  (bind _game_instance (`self.Game Instance`))
  (`/Engine/EditorBlueprintResources/StandardMacros.IsValid` (`self.Game Instance`)
    (:`Is Valid`
      (bind _output_get (set `/Game/ShootingGame/GameMode/ShootingGameInstance.Player Count` (+ (`/Game/ShootingGame/GameMode/ShootingGameInstance.Player Count` _game_instance) 1) _game_instance))
      (`KismetSystemLibrary.PrintString` (`KismetStringLibrary.Conv_IntToString` _output_get) false false (struct :`R` 0.598702 :`G` 0.03805 :`B` 1.0 :`A` 1.0) 30.0))
    (:`Is Not Valid`
      (`KismetSystemLibrary.K2_SetTimer` null "Set Player Count" 0.1))))

(fn `UserConstructionScript`)