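; BP_Weapon_Once is a weapon Blueprint for the shooting game that overrides setup and trigger behavior from its parent.
; On BeginPlay it runs the parent logic, then sets the camera shake to the rocket launcher variant.
; PullTrigger checks ammo, plays the rifle fire montage on the owning character and sets a large recoil vector along the camera's forward direction.
; The graph itself spawns no projectile and applies no recoil.
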(event `self.ReceiveBeginPlay`
  (`parent.ReceiveBeginPlay`)
  (set `self.Camera Shake` "/Game/ShootingGame/ShootShakeCamera_RocketLauncher.ShootShakeCamera_RocketLauncher_C"))

(fn `PullTrigger`
  (params (Character :type "Character Object Reference"))
  (if (`self.Can Use Ammo`)
    (`Character.PlayAnimMontage` (`self.Own Character`) "/Game/ShootingGame/Animation/My_Fire_Reload_Equip_Jump/AM_Rifle_Fire.AM_Rifle_Fire" 1.0 "None")
    (set `self.Recoil Vector` (* (`self.GetActorForwardVector` (`GameplayStatics.GetPlayerCameraManager` 0)) 100000.0))))

(fn `UserConstructionScript`
  (`parent.UserConstructionScript`))