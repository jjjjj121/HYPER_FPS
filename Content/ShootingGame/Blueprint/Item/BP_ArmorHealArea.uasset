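; BP_ArmorHealArea is an area item that restores armor to living BP_HyperCharacter actors inside its Box.
; AddHealLoop gets the Box's overlapping characters, skips dead ones and calls AddArmor with AddHealValue on each one's BP_ShootingPlayerState.
; The event graph holds only disabled stubs, so nothing in this Blueprint's own graphs calls AddHealLoop.
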(fn `Add Heal Loop`
  (for _array_element (`PrimitiveComponent.GetOverlappingActors` (`self.Box`) "/Game/ShootingGame/GameMode/BP_HyperCharacter.BP_HyperCharacter_C")
    (bind _asbp_hyper_character_a (cast `/Game/ShootingGame/GameMode/BP_HyperCharacter` _array_element))
    (if (not (`/Game/ShootingGame/GameMode/BP_HyperCharacter.Is Die` _asbp_hyper_character_a))
      (bind _asbp_shooting_player_state (cast `/Game/ShootingGame/GameMode/BP_ShootingPlayerState` (`Pawn.PlayerState` _asbp_hyper_character_a)))
      (`/Game/ShootingGame/GameMode/BP_ShootingPlayerState.Add Armor` _asbp_shooting_player_state (`self.Add Heal Value`)))))

(fn `UserConstructionScript`
  (`parent.UserConstructionScript`))