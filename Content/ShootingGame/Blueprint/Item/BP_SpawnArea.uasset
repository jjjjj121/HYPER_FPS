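; BP_SpawnArea is an item spawner that scatters 15 items across a large navigable radius around itself after a short delay at BeginPlay.
; SpawnItem runs only with authority, picks a random navmesh point, traces down to static ground with debug drawing, spawns slightly above it, and recursively retries on a miss.
; DestroyItem and RandomSpawn schedule further spawns on randomized timers.
; The DelayForLoop macro delays once before looping, not between iterations.
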(event `self.ReceiveBeginPlay`
  (`self.Delay For loop` 1 15 0.6
    (:`Loop Body`
      (`self.Spawn Item`))))

(fn `Destroy Item`
  (params (DestroyedActor :type "Actor Object Reference"))
  (`KismetSystemLibrary.K2_SetTimer` null "Spawn Item" (`KismetMathLibrary.Conv_IntToDouble` (`KismetMathLibrary.RandomIntegerInRange` 10 20))))

(fn `Random Spawn`
  (`KismetSystemLibrary.K2_SetTimer` null "Spawn Item" (`KismetMathLibrary.Conv_IntToDouble` (`KismetMathLibrary.RandomIntegerInRange` 1 5))))

(fn `Spawn Item`
  (bind (_returnvalue_location _returnvalue_rotation _returnvalue_scale) (`KismetMathLibrary.BreakTransform` (`self.GetTransform`)))
  (bind (_returnvalue_x _returnvalue_y _returnvalue_z) (`KismetMathLibrary.BreakVector` (`self.K2_GetActorLocation`)))
  (`/Engine/EditorBlueprintResources/ActorMacros.Switch Has Authority`
    (:`Authority`
      (bind _randomlocation (`NavigationSystemV1.K2_GetRandomLocationInNavigableRadius` (`KismetMathLibrary.MakeVector` _returnvalue_x _returnvalue_y _returnvalue_z) 7000.0 null null))
      (bind (_outhit _returnvalue) (`KismetSystemLibrary.LineTraceSingleForObjects` :`Start` _randomlocation :`End` (`KismetMathLibrary.MakeVector` (.x _randomlocation) (.y _randomlocation) -100000.0) :`ObjectTypes` (`|MakeArray` "ObjectTypeQuery1" :!type "EObjectTypeQuery Enum") :`DrawDebugType` "ForDuration"))
      (if _returnvalue
        (bind _returnvalue_2 (`|SpawnActorFromClass` (`self.Items`) (`KismetMathLibrary.MakeTransform` (`KismetMathLibrary.MakeVector` (.x (`.Location` (`GameplayStatics.BreakHitResult` _outhit))) (.y (`.Location` (`GameplayStatics.BreakHitResult` _outhit))) (+ (.z (`.Location` (`GameplayStatics.BreakHitResult` _outhit))) 100.0)) _returnvalue_rotation _returnvalue_scale) "AdjustIfPossibleButAlwaysSpawn" "OverrideRootScale" null self null))
        (set `self.Spawned Item` _returnvalue_2)
        (else
          (`self.Spawn Item`))))))

(fn `UserConstructionScript`)