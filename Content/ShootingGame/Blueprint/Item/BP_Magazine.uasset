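; BP_Magazine is an ammo magazine item that adds a magazine to the character who uses it.
; While its static mesh is visible, Tick spins it around the yaw axis at a constant, frame-rate-independent speed.
; UseItem runs the parent check first; on success it casts the user to BP_HyperCharacter, calls AddMag, then destroys the actor.
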(event `self.ReceiveBeginPlay`
  (`parent.ReceiveBeginPlay`))

(event `self.ReceiveTick`
  (params (DeltaSeconds :type "Float (single-precision)"))
  (bind _staticmesh (`self.StaticMesh`))
  (if (`SceneComponent.IsVisible` _staticmesh)
    (`SceneComponent.K2_AddRelativeRotation` _staticmesh (`KismetMathLibrary.MakeRotator` 0.0 0.0 (* DeltaSeconds 150.0)) false false)))

(fn `UseItem`
  (params (character :type "Character Object Reference"))
  (bind _can_use_ (`parent.UseItem` character))
  (if _can_use_
    (bind _asbp_hyper_character (cast `/Game/ShootingGame/GameMode/BP_HyperCharacter` character))
    (`/Game/ShootingGame/GameMode/BP_HyperCharacter.Add Mag` _asbp_hyper_character)
    (`self.K2_DestroyActor`)))

(fn `UserConstructionScript`)