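; BP_HPHealArea is a healing zone actor that periodically restores health to living BP_HyperCharacter actors inside its box.
; A looping one-second timer queries the box's overlapping characters and calls AddHeal on each one's BP_ShootingPlayerState with AddHealValue.
; Box overlap begin and end events switch a Niagara effect on and off, without filtering by actor or counting occupants.
; Tick continuously spins the static mesh around its yaw axis.
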(event `self.ReceiveTick`
  (params (DeltaSeconds :type "Float (single-precision)"))
  (`SceneComponent.K2_AddRelativeRotation` (`self.StaticMesh`) (`KismetMathLibrary.MakeRotator` 0.0 0.0 (* DeltaSeconds 100.0)) false false))

(event `self.ReceiveBeginPlay`
  (`ActorComponent.Deactivate` (`self.Niagara1`))
  (`KismetSystemLibrary.K2_SetTimer` null "Add Heal Loop" 1.0 true))

(event `self.Box.OnComponentBeginOverlap`
  (params (OverlappedComponent :type "PrimitiveComponent Object Reference") (OtherActor :type "Actor Object Reference") (OtherComp :type "PrimitiveComponent Object Reference") (OtherBodyIndex :type Integer) (bFromSweep :type Boolean) (SweepResult :type "HitResult Structure (by ref)"))
  (`ActorComponent.Activate` (`self.Niagara1`) false))

(event `self.Box.OnComponentEndOverlap`
  (params (OverlappedComponent :type "PrimitiveComponent Object Reference") (OtherActor :type "Actor Object Reference") (OtherComp :type "PrimitiveComponent Object Reference") (OtherBodyIndex :type Integer))
  (`ActorComponent.Deactivate` (`self.Niagara1`)))

(fn `Add Heal Loop`
  (for _array_element (`PrimitiveComponent.GetOverlappingActors` (`self.Box`) "/Game/ShootingGame/GameMode/BP_HyperCharacter.BP_HyperCharacter_C")
    (bind _asbp_hyper_character_a (cast `/Game/ShootingGame/GameMode/BP_HyperCharacter` _array_element))
    (if (not (`/Game/ShootingGame/GameMode/BP_HyperCharacter.Is Die` _asbp_hyper_character_a))
      (bind _asbp_shooting_player_state (cast `/Game/ShootingGame/GameMode/BP_ShootingPlayerState` (`Pawn.PlayerState` _asbp_hyper_character_a)))
      (`/Game/ShootingGame/GameMode/BP_ShootingPlayerState.Add Heal` _asbp_shooting_player_state (`self.Add Heal Value`)))))

(fn `UserConstructionScript`)