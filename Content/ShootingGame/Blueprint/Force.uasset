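; Force is a shooting-game actor that deals a one-shot burst of radial damage at its own location when spawned.
; On BeginPlay, only the authority applies full damage within a small radius and draws two larger debug spheres that do not match that radius.
; Radial force impulse, falloff damage with an instigator, direct damage and delayed self-destruction are all left disconnected, so the actor never destroys itself.
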(event `self.ReceiveBeginPlay`
  (bind _returnvalue (`self.K2_GetActorLocation`))
  (`/Engine/EditorBlueprintResources/ActorMacros.Switch Has Authority`
    (:`Authority`
      (`GameplayStatics.ApplyRadialDamage` :`BaseDamage` 100.0 :`Origin` _returnvalue :`DamageRadius` 50.0 :`DamageTypeClass` "/Script/Engine.DamageType" :`DamageCauser` null :`InstigatedByController` null :`bDoFullDamage` true)
      (`KismetSystemLibrary.DrawDebugSphere` _returnvalue 250.0 24 (struct :`R` 1.0 :`G` 1.0 :`B` 1.0 :`A` 1.0) 2.0 1.0)
      (`KismetSystemLibrary.DrawDebugSphere` _returnvalue 500.0 24 (struct :`R` 1.0 :`G` 1.0 :`B` 1.0 :`A` 1.0) 2.0 1.0))))

(fn `UserConstructionScript`)