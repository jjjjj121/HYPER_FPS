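; BP_RotateBox is an interactable box actor whose Cube can be toggled to spin around its yaw axis.
; EventPress calls EnablePlay to flip IsPlay, and Tick adds a fixed yaw step while it is true, so speed depends on frame rate.
; EventCanPickUp, EventPress and EventRelease all return false.
; Overlap events are empty, with input-toggling and authority-check nodes left disconnected.
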(event `self.ReceiveTick`
  (params (DeltaSeconds :type "Float (single-precision)"))
  (if (`self.Is Play?`)
    (`SceneComponent.K2_AddRelativeRotation` (`self.Cube`) (`KismetMathLibrary.MakeRotator` 0.0 0.0 5.0) false false)))

(event `self.Cube.OnComponentBeginOverlap`
  (params (OverlappedComponent :type "PrimitiveComponent Object Reference") (OtherActor :type "Actor Object Reference") (OtherComp :type "PrimitiveComponent Object Reference") (OtherBodyIndex :type Integer) (bFromSweep :type Boolean) (SweepResult :type "HitResult Structure (by ref)"))
  ;[1 1 1] 내가한거
)

(event `self.Cube.OnComponentEndOverlap`
  (params (OverlappedComponent :type "PrimitiveComponent Object Reference") (OtherActor :type "Actor Object Reference") (OtherComp :type "PrimitiveComponent Object Reference") (OtherBodyIndex :type Integer))
  ;[1 1 1] 내가한거
)

(event `InputAction|PickUp`
  (params (Key :type "Key Structure")))

(fn `EnablePlay`
  (set `self.Is Play?` (not (`self.Is Play?`))))

(fn `EventCanPickUp`
  (returns (`Can Pick UP?` :type Boolean))
  (return false))

(fn `EventPress`
  (params (Character :type "Character Object Reference"))
  (returns (Result :type Boolean))
  (`self.EnablePlay`)
  (return false))

(fn `EventRelease`
  (params (Character :type "Character Object Reference"))
  (returns (Result :type Boolean))
  (return false))

(fn `UserConstructionScript`)