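; BP_Counter is a counter actor in the shooting game that raises its count each time it is pressed and shows it on a TextRender.
; EventPress calls CountUp, which increments Count and updates the text.
; EventCanPickUp returns false, and EventRelease does nothing but return false.
; The Cube overlap events are empty, leaving disconnected logic that would toggle input for BP_HyperCharacter and count up directly.
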(event `self.Cube.OnComponentBeginOverlap`
  (params (OverlappedComponent :type "PrimitiveComponent Object Reference") (OtherActor :type "Actor Object Reference") (OtherComp :type "PrimitiveComponent Object Reference") (OtherBodyIndex :type Integer) (bFromSweep :type Boolean) (SweepResult :type "HitResult Structure (by ref)"))
  ;[1 1 1] 내가한거
)

(event `self.Cube.OnComponentEndOverlap`
  (params (OverlappedComponent :type "PrimitiveComponent Object Reference") (OtherActor :type "Actor Object Reference") (OtherComp :type "PrimitiveComponent Object Reference") (OtherBodyIndex :type Integer))
  ;[1 1 1] 내가한거
)

(event `InputAction|PickUp`
  (params (Key :type "Key Structure")))

(fn `CountUp`
  (bind _result (`/Engine/EditorBlueprintResources/StandardMacros.IncrementFloat` (`self.Count`))
    (:`  `
      (`TextRenderComponent.K2_SetText` (`self.TextRender`) (`KismetTextLibrary.Conv_DoubleToText` _result "HalfToEven")))))

(fn `EventCanPickUp`
  (returns (`Can Pick UP?` :type Boolean))
  (return false))

(fn `EventPress`
  (params (Character :type "Character Object Reference"))
  (returns (Result :type Boolean))
  (`self.CountUp`)
  (return false))

(fn `EventRelease`
  (params (Character :type "Character Object Reference"))
  (returns (Result :type Boolean))
  (return false))

(fn `UserConstructionScript`)