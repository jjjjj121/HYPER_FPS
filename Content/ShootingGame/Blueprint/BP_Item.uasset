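; BP_Item is a pickup item base that fires UseItem when a Character overlaps its static mesh.
; UseItem only validates: it returns true on the authority for a living BP_HyperCharacter, with no effect applied here.
; When destroyed, the item passes its OwnSpawner to BP_HyperFPSGameMode's CheckSpawnItem, using the game mode reference cached at BeginPlay.
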(event `self.ReceiveBeginPlay`
  (bind _asbp_hyper_fpsgame_mode (cast `/Game/ShootingGame/GameMode/MultiPlay/BP_HyperFPSGameMode` (`GameplayStatics.GetGameMode`)))
  (set `self.Game Mode` _asbp_hyper_fpsgame_mode))

(event `self.StaticMesh.OnComponentBeginOverlap`
  (params (OverlappedComponent :type "PrimitiveComponent Object Reference") (OtherActor :type "Actor Object Reference") (OtherComp :type "PrimitiveComponent Object Reference") (OtherBodyIndex :type Integer) (bFromSweep :type Boolean) (SweepResult :type "HitResult Structure (by ref)"))
  (bind _ascharacter (cast `Character` OtherActor))
  (`self.UseItem` _ascharacter))

(event `self.ReceiveDestroyed`
  (`/Game/ShootingGame/GameMode/MultiPlay/BP_HyperFPSGameMode.Check Spawn Item` (`self.Game Mode`) (`self.Own Spawner`)))

(fn `UseItem`
  (params (character :type "Character Object Reference"))
  (returns (`Can Use?` :type Boolean))
  (`/Engine/EditorBlueprintResources/ActorMacros.Switch Has Authority`
    (:`Authority`
      (bind _asbp_hyper_character (cast `/Game/ShootingGame/GameMode/BP_HyperCharacter` character))
      (if (`/Game/ShootingGame/GameMode/BP_HyperCharacter.Is Die` _asbp_hyper_character)
        (return false)
        (else
          (return true))))
    (:`Remote`
      (return false))))

(fn `UserConstructionScript`)