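; Networked rifle pickup that attaches to BP_HyperCharacter, taking its mesh, ammo capacity and damage from WeaponRef.
; A looping timer replays fire montages, while notify events trigger effects, owner-only recoil and shot or reload requests.
; ServerHitCheck spends ammo and line-traces from the camera, widening spread during unzoomed sustained fire, then damages actors and destructibles.
; Recoil recovers by timer, ammo updates the HUD, and aiming blends the view to the weapon.
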(event `self.ReceiveBeginPlay`
  (bind (_weaponref_weaponclass _weaponref_staticmesh _weaponref_maxammo) (break `/Game/ShootingGame/Data/ST_Weapon` (`self.WeaponRef`)))
  (`StaticMeshComponent.SetStaticMesh` (`self.StaticMesh`) _weaponref_staticmesh)
  (set `self.Ammo` _weaponref_maxammo))

(event `ReqHitCheck`
  (params (Location :type "Vector Structure") (`Forward Vector` :type "Vector Structure"))
  (`KismetSystemLibrary.PrintString` "ReqHitCheck" false false)
  (`self.Server Hit Check` Location `Forward Vector`))

(event `ReqReload`
  (`self.Server Use Mag`))

(event `ResImpactEffect`
  (params (`Impact Loaction` :type "Vector Structure"))
  (`self.Spawn Impact Effect` `Impact Loaction`))

(event `Destructible Damage`
  (params (Wall :type "DestructibleComponent Object Reference") (Damage :type "Float (double-precision)") (`Hit Location` :type "Vector Structure") (`Impulse Dir` :type "Vector Structure"))
  (`DestructibleComponent.ApplyDamage` Wall Damage `Hit Location` `Impulse Dir` 3000.0))

(event `Move Trace`
  (params (`Impact Point` :type "Vector Structure"))
  (bind _staticmesh (`self.StaticMesh`))
  (`GameplayStatics.SpawnEmitterAtLocation` "/Game/MilitaryWeapDark/FX/P_AssaultRifle_Tracer_01.P_AssaultRifle_Tracer_01" (`SceneComponent.GetSocketLocation` _staticmesh "muzzle") (`SceneComponent.GetSocketRotation` _staticmesh "muzzle") (0.5 1.0 1.0)))

(fn `Add Recoil`
  (if (not (`/Game/ShootingGame/GameMode/BP_HyperCharacter.Is Death` (`self.Own Character`)))
    (`self.Check My Owner`
      (:`True`
        (`PlayerController.AddPitchInput` (`GameplayStatics.GetPlayerController` 0) (* (`self.Recoil Value`) -1.0))
        (`self.ShakeCamera`)))))

(fn `AddShoot`
  (locals (`Shoot Count` :type "Float (double-precision)"))
  (set `self.ShootCount` (+ (`self.ShootCount`) 1))
  (if (`self.Can Use Ammo`)
    (`/Engine/EditorBlueprintResources/StandardMacros.IsValid` (`self.Own Character`)
      (:`Is Valid`
        (`Character.PlayAnimMontage` (`self.Own Character`) "/Game/ShootingGame/Animation/My_Fire_Reload_Equip_Jump/AM_Rifle_Fire.AM_Rifle_Fire" 1.0 "None")))
    (else
      (`KismetSystemLibrary.K2_ClearTimer` null "AddShoot")
      (`self.Reset Recoil`)
      (set `self.ShootCount` 0))))

(fn `AttachToCharacter`
  (params (Character :type "Character Object Reference"))
  (bind _staticmesh (`self.StaticMesh`))
  (bind _asbp_hyper_character (cast `/Game/ShootingGame/GameMode/BP_HyperCharacter` Character))
  (set `self.Own Character` _asbp_hyper_character)
  (set `/Game/ShootingGame/GameMode/BP_HyperCharacter.Attached Weapon` self _asbp_hyper_character)
  (set `Pawn.bUseControllerRotationYaw` true _asbp_hyper_character)
  (set `CharacterMovementComponent.bOrientRotationToMovement` false (`Character.CharacterMovement` _asbp_hyper_character))
  (`Character.PlayAnimMontage` _asbp_hyper_character "/Game/RifleAnimsetPro/Animations/EquipRifle_Montage.EquipRifle_Montage" 1.0 "None")
  (`PrimitiveComponent.SetSimulatePhysics` _staticmesh false)
  (`PrimitiveComponent.SetCollisionEnabled` _staticmesh "NoCollision")
  (`self.K2_AttachToComponent` (`Character.Mesh` Character) "weapon" "SnapToTarget" "SnapToTarget" "KeepWorld") ; Actorr가 Component에 붙음
  (`self.Update UI` (`self.Ammo`)))

(fn `Can Use Ammo`
  (returns (`Can Use` :type Boolean))
  (return (> (`self.Ammo`) 0)))

(fn `Check Cur Info`
  (returns (`Cur Data` :type Integer) (`Default Data` :type Integer))
  (bind (_weaponref_weaponclass _weaponref_staticmesh _weaponref_maxammo) (break `/Game/ShootingGame/Data/ST_Weapon` (`self.WeaponRef`)))
  (return (`self.Ammo`) _weaponref_maxammo))

(fn `DetachToCharacter`
  (params (Character :type "Character Object Reference"))
  (bind _staticmesh (`self.StaticMesh`))
  (`PrimitiveComponent.SetCollisionEnabled` _staticmesh "QueryAndPhysics")
  (`PrimitiveComponent.SetSimulatePhysics` _staticmesh true)
  (`self.Update UI` 0)
  ;[1 1 1] UnEquip 상태로 정보 변경
  (bind _asbp_hyper_character (cast `/Game/ShootingGame/GameMode/BP_HyperCharacter` Character))
  (set `/Game/ShootingGame/GameMode/BP_HyperCharacter.Attached Weapon` null _asbp_hyper_character)
  (set `self.Own Character` null)
  (set `Pawn.bUseControllerRotationYaw` false _asbp_hyper_character)
  (set `CharacterMovementComponent.bOrientRotationToMovement` true (`Character.CharacterMovement` _asbp_hyper_character))
  (if (`/Game/ShootingGame/GameMode/BP_HyperCharacter.Is Death` _asbp_hyper_character)
    (`self.K2_DetachFromActor` "KeepWorld" "KeepWorld" "KeepWorld")))

(fn `EventCanPickUp`
  (returns (`Can Pick UP?` :type Boolean))
  (return (not (`KismetSystemLibrary.IsValid` (`self.Own Character`)))))

(fn `EventNotify Start Reload`
  (params (Character :type "Character Object Reference"))
  (`AudioComponent.Play` (`self.Rifle_Reload_Cue`) 0.0)
  (`self.Check My Owner`
    (:`True`
      (bind _output_get (set `self.Ammo` 0))
      (`self.Update UI` _output_get))))

(fn `EventNotifyFire`
  (params (character :type "Character Object Reference"))
  (bind _returnvalue (`GameplayStatics.GetPlayerCameraManager` 0))
  (bind _staticmesh (`self.StaticMesh`))
  ;[1 1 1] Client
  (`/Engine/EditorBlueprintResources/ActorMacros.Switch Has Authority`
    (:`Authority`
      (if (`self.Can Use Ammo`)
        (`GameplayStatics.SpawnEmitterAttached` (`self.Spawn Emitter`) _staticmesh "muzzle" (`SceneComponent.GetSocketLocation` _staticmesh "muzzle") (`SceneComponent.GetSocketRotation` _staticmesh "muzzle") (1.0 1.0 1.0) "KeepWorldPosition" :!label _label)
        (`AudioComponent.Play` (`self.Shoot Audio`) 0.0)
        (`self.Check My Owner`
          (:`True`
            (`self.Add Recoil`)
            (`KismetSystemLibrary.PrintString` "EventNotifyFire" false false)
            (`self.ReqHitCheck` (`PlayerCameraManager.GetCameraLocation` _returnvalue) (`self.GetActorForwardVector` _returnvalue))))))
    (:`Remote`
      (bind _isusedammo (`self.Use Ammo`))
      (if _isusedammo
        (goto _label)))))

(fn `EventNotifyReload`
  (params (character :type "Character Object Reference"))
  (`self.Check My Owner`
    (:`True`
      (`self.ReqReload`))))

(fn `EventPress`
  (params (Character :type "Character Object Reference"))
  (returns (Result :type Boolean))
  (bind _asbp_hyper_character (cast `/Game/ShootingGame/GameMode/BP_HyperCharacter` Character))
  (bind _attached_weapon (`/Game/ShootingGame/GameMode/BP_HyperCharacter.Attached Weapon` _asbp_hyper_character))
  (`/Engine/EditorBlueprintResources/StandardMacros.IsValid` _attached_weapon
    (:`Is Valid`
      (`self.DetachToCharacter` _attached_weapon Character))
    (:`Is Not Valid`
      _))
  (`self.AttachToCharacter` Character)
  (return true))

(fn `EventRelease`
  (params (Character :type "Character Object Reference"))
  (returns (Result :type Boolean))
  (return true))

(fn `Holster`
  (bind _asbp_hyper_character (cast `/Game/ShootingGame/GameMode/BP_HyperCharacter` (`GameplayStatics.GetPlayerPawn` 0)))
  (`PrimitiveComponent.AddImpulse` (`self.StaticMesh`) (* (`SceneComponent.GetForwardVector` (`/Game/ShootingGame/GameMode/BP_HyperCharacter.Throw Direction` _asbp_hyper_character)) 700.0) "None" true))

(fn `OnRep_Ammo`
  (`self.Update UI` (`self.Ammo`)))

(fn `PullTrigger`
  (params (Character :type "Character Object Reference"))
  (if (`self.Can Use Ammo`)
    (set `self.ShootCount` (+ (`self.ShootCount`) 1))
    (`Character.PlayAnimMontage` (`self.Own Character`) "/Game/ShootingGame/Animation/My_Fire_Reload_Equip_Jump/AM_Rifle_Fire.AM_Rifle_Fire" 1.0 "None")
    (`KismetSystemLibrary.K2_SetTimer` null "AddShoot" 0.1 true)
    (set `self.Recoil Vector` (* (`self.GetActorForwardVector` (`GameplayStatics.GetPlayerCameraManager` 0)) 100000.0))))

(fn `Recoil`
  (`/Engine/EditorBlueprintResources/StandardMacros.IsValid` (`self.Own Character`)
    (:`Is Valid`
      (if (`/Game/ShootingGame/GameMode/BP_HyperCharacter.Is Death` (`self.Own Character`))
        _
        (elif (`self.Should Reset Recoil?`)
          (`KismetSystemLibrary.PrintString` "Reset" false false)
          (`PlayerController.AddPitchInput` (`GameplayStatics.GetPlayerController` 0) 0.1)
          (else
            (`KismetSystemLibrary.K2_ClearTimer` null "Recoil")))))))

(fn `Release Trigger`
  (if (`self.Can Use Ammo`)
    (if (`self.Should Reset Recoil?`)
      (`self.Reset Recoil`))
    (`KismetSystemLibrary.K2_ClearTimer` null "AddShoot")
    (set `self.Is Reloading?` false)
    (set `self.ShootCount` 0)))

(fn `Reload`
  (bind (_weaponref_weaponclass _weaponref_staticmesh _weaponref_maxammo) (break `/Game/ShootingGame/Data/ST_Weapon` (`self.WeaponRef`)))
  (if (and (< (`self.Ammo`) _weaponref_maxammo) (`/Game/ShootingGame/GameMode/BP_HyperCharacter.Has Mag` (`self.Own Character`)))
    (`Character.PlayAnimMontage` (`self.Own Character`) "/Game/ShootingGame/Animation/My_Fire_Reload_Equip_Jump/AS_Rifle_ReloadLoaded_Montage.AS_Rifle_ReloadLoaded_Montage" 1.0 "None")))

(fn `Reset Recoil`
  (`KismetSystemLibrary.K2_SetTimer` null "Recoil" (`self.Recoil Speed`) true))

(fn `Server Hit Check`
  (params (Location :type "Vector Structure") (`Forward Vector` :type "Vector Structure"))
  (bind (_weaponref_weaponclass _weaponref_staticmesh _weaponref_maxammo _weaponref_damage) (break `/Game/ShootingGame/Data/ST_Weapon` (`self.WeaponRef`)))
  (bind (_weaponref_weaponclass_2 _weaponref_staticmesh_2 _weaponref_maxammo_2 _weaponref_damage_2) (break `/Game/ShootingGame/Data/ST_Weapon` (`self.WeaponRef`)))
  (bind (_weaponref_weaponclass_3 _weaponref_staticmesh_3 _weaponref_maxammo_3 _weaponref_damage_3) (break `/Game/ShootingGame/Data/ST_Weapon` (`self.WeaponRef`)))
  (bind (_weaponref_weaponclass_4 _weaponref_staticmesh_4 _weaponref_maxammo_4 _weaponref_damage_4) (break `/Game/ShootingGame/Data/ST_Weapon` (`self.WeaponRef`)))
  (bind _returnvalue (+ Location (* `Forward Vector` 300.0)))
  (bind _isusedammo (`self.Use Ammo`))
  (if _isusedammo
    (if (`/Game/ShootingGame/GameMode/BP_HyperCharacter.Is Zoom?` (`self.Own Character`))
      (bind _outhit (`KismetSystemLibrary.LineTraceSingleForObjects` :`Start` _returnvalue :`End` (+ Location (* `Forward Vector` 10000.0)) :`ObjectTypes` (`|MakeArray` "ObjectTypeQuery1" "ObjectTypeQuery2" "ObjectTypeQuery3" "ObjectTypeQuery4" "ObjectTypeQuery5" "ObjectTypeQuery6" :!type "EObjectTypeQuery Enum") :`DrawDebugType` "ForDuration"))
      (bind (_bblockinghit _binitialoverlap _time _distance _location _impactpoint _normal _impactnormal _physmat _hitactor _hitcomponent _hitbonename _hititem _elementindex _faceindex _tracestart _traceend) (`GameplayStatics.BreakHitResult` _outhit))
      (`GameplayStatics.SpawnEmitterAtLocation` "/Game/MilitaryWeapDark/FX/P_Impact_Metal_Medium_01.P_Impact_Metal_Medium_01" _location)
      (`|ExecutionSequence`
        (:`then_0`
          (`GameplayStatics.ApplyDamage` _hitactor _weaponref_damage (`Pawn.GetController` (`self.Own Character`)) self) ; 번개표시 = 서버에서만 실행
          (`self.ResImpactEffect` _location))
        (:`then_1`
          (bind _asdestructible_component (cast `DestructibleComponent` _hitcomponent))
          (`self.Destructible Damage` _asdestructible_component _weaponref_damage_2 _location _impactpoint)))
      (else
        (bind _outhit_2 (`KismetSystemLibrary.LineTraceSingleForObjects` :`Start` _returnvalue :`End` (+ Location (* (`KismetMathLibrary.RandomUnitVectorInConeInDegrees` `Forward Vector` (`KismetMathLibrary.FClamp` (* (`self.ShootCount`) 0.5) 0.0 5.0)) 10000.0)) :`ObjectTypes` (`|MakeArray` "ObjectTypeQuery1" "ObjectTypeQuery2" "ObjectTypeQuery3" "ObjectTypeQuery4" "ObjectTypeQuery5" "ObjectTypeQuery6" :!type "EObjectTypeQuery Enum") :`DrawDebugType` "ForDuration"))
        (bind (_bblockinghit_2 _binitialoverlap_2 _time_2 _distance_2 _location_2 _impactpoint_2 _normal_2 _impactnormal_2 _physmat_2 _hitactor_2 _hitcomponent_2) (`GameplayStatics.BreakHitResult` _outhit_2))
        (`GameplayStatics.SpawnEmitterAtLocation` "/Game/MilitaryWeapDark/FX/P_Impact_Metal_Medium_01.P_Impact_Metal_Medium_01" _location_2)
        (`|ExecutionSequence`
          (:`then_0`
            (`GameplayStatics.ApplyDamage` _hitactor_2 _weaponref_damage_3 (`Pawn.GetController` (`self.Own Character`)) self) ; 번개표시 = 서버에서만 실행
            (`self.ResImpactEffect` _location_2))
          (:`then_1`
            (bind _asdestructible_component_2 (cast `DestructibleComponent` _hitcomponent_2))
            (`self.Destructible Damage` _asdestructible_component_2 _weaponref_damage_4 _location_2 _impactpoint_2)
            (`KismetSystemLibrary.PrintString` "Destructible Damage" false false (struct :`G` 0.66 :`B` 1.0 :`A` 1.0) 5.0)))))))

(fn `Server Use Mag`
  (`AudioComponent.Play` (`self.Rifle_ReloadInsert_Cue`) 0.0)
  (`self.Set Ammo`))

(fn `Set Ammo`
  (bind (_weaponref_weaponclass _weaponref_staticmesh _weaponref_maxammo) (break `/Game/ShootingGame/Data/ST_Weapon` (`self.WeaponRef`)))
  (bind _is_used_mag (`/Game/ShootingGame/GameMode/BP_HyperCharacter.UseMag` (`self.Own Character`)))
  (if _is_used_mag
    (bind _output_get (set `self.Ammo` _weaponref_maxammo))
    (`self.Update UI` _output_get)))

(fn `ShakeCamera`
  (`PlayerController.ClientStartCameraShake` :`self` (`GameplayStatics.GetPlayerController` 0) :`Shake` (`self.Camera Shake`) :`Scale` (`self.Shake Camera Scale`)))

(fn `Should Reset Recoil?`
  (returns (ReturnValue :type Boolean))
  (bind (_recoil_vector_x _recoil_vector_y _recoil_vector_z) (`KismetMathLibrary.BreakVector` (`self.Recoil Vector`)))
  (bind (_returnvalue_x _returnvalue_y _returnvalue_z) (`KismetMathLibrary.BreakVector` (* (`self.GetActorForwardVector` (`GameplayStatics.GetPlayerCameraManager` 0)) 100000.0)))
  (return (> _returnvalue_z _recoil_vector_z)))

(fn `Spawn Impact Effect`
  (params (`Impact Loaction` :type "Vector Structure"))
  (bind _returnvalue (`SceneComponent.GetSocketLocation` (`self.StaticMesh`) "muzzle"))
  (`GameplayStatics.SpawnEmitterAtLocation` "/Game/MilitaryWeapDark/FX/P_Impact_Metal_Medium_01.P_Impact_Metal_Medium_01" `Impact Loaction`)
  (`|SpawnActorFromClass` "/Game/ShootingGame/Blueprint/Weapon/Original_Projectile.Original_Projectile_C" (`KismetMathLibrary.MakeTransform` _returnvalue (`KismetMathLibrary.FindLookAtRotation` _returnvalue `Impact Loaction`)) "Undefined" "OverrideRootScale" null null))

(fn `SpawnEmitter`
  (params (Character :type "Character Object Reference"))
  (bind _staticmesh (`self.StaticMesh`))
  (`GameplayStatics.SpawnEmitterAttached` "/Game/MilitaryWeapDark/FX/P_AssaultRifle_MuzzleFlash.P_AssaultRifle_MuzzleFlash" _staticmesh "muzzle" (`SceneComponent.GetSocketLocation` _staticmesh "muzzle") (`SceneComponent.GetSocketRotation` _staticmesh "muzzle") (1.0 1.0 1.0) "KeepWorldPosition")
  (`AudioComponent.Play` (`self.Shoot Audio`) 0.0))

(fn `Toggle Aim`
  (params (Character :type "/Game/ShootingGame/GameMode/BP_HyperCharacter Object Reference") (`Is Press?` :type Boolean))
  (returns (`Toggle Aim` :type Boolean))
  (if `Is Press?`
    (`PlayerCameraManager.StartCameraFade` :`self` (`PlayerController.PlayerCameraManager` (`GameplayStatics.GetPlayerController` 0)) :`FromAlpha` 1.0 :`Duration` 2.0)
    (`PlayerController.SetViewTargetWithBlend` (`GameplayStatics.GetPlayerController` 0) self 0.3 "VTBlend_Linear" 0.0 false)
    (return true)
    (else
      (`PlayerController.SetViewTargetWithBlend` (`GameplayStatics.GetPlayerController` 0) Character 0.3 "VTBlend_Linear" 0.0 false)
      (return false))))

(fn `Update UI`
  (params (Ammo :type Integer))
  (bind (_weaponref_weaponclass _weaponref_staticmesh _weaponref_maxammo) (break `/Game/ShootingGame/Data/ST_Weapon` (`self.WeaponRef`)))
  (`/Engine/EditorBlueprintResources/StandardMacros.IsValid` (`self.Own Character`)
    (:`Is Valid`
      (`self.Check My Owner`
        (:`True`
          (`/Inventory3/InventorySystem/ActorComponent/ItemTemplatePickupComponent.UpdateAmmo` (`/Game/ShootingGame/GameMode/BP_HyperCharacter.TemplatePickupComponent` (`self.Own Character`)) Ammo _weaponref_maxammo)
          (bind _asbp_shooting_hud (cast `/Game/ShootingGame/GameMode/BP_ShootingHUD` (`PlayerController.GetHUD` (`GameplayStatics.GetPlayerController` 0))))
          (`/Game/ShootingGame/GameMode/BP_ShootingHUD.UpdateAmmo` _asbp_shooting_hud Ammo))))))

(fn `Use Ammo`
  (returns (IsUsedAmmo :type Boolean))
  (if (`self.Can Use Ammo`)
    (bind _output_get (set `self.Ammo` (- (`self.Ammo`) 1)))
    (`self.Update UI` _output_get)
    (return true)
    (else
      (return false))))

(fn `UserConstructionScript`)

(fn `Zoom`
  (params (`delta value` :type "Float (double-precision)") (`Zoom In?` :type Boolean))
  (returns (NewParam1 :type Boolean)))