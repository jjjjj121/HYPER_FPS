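; Weapon spawner actor that scatters 15 random weapons around itself when play begins, with spawning done only on the server.
; A custom loop macro waits once briefly, then calls SpawnActor for every iteration without further delay.
; Each call picks a random navmesh point, traces down to static world geometry and spawns a random T_Weapon row's class just above the hit.
; The fixed-weapon lineup and SpawnArmorFunc are inactive or empty.
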(event `self.ReceiveBeginPlay`
  (`self.Delay For loop` 1 15 0.6
    (:`Loop Body`
      (`self.Spawn Actor`))))

(fn `Get Random Weapon Name`
  (returns (WeaponName :type "Name (by ref)"))
  (bind _outrownames (`DataTableFunctionLibrary.GetDataTableRowNames` "/Game/ShootingGame/Data/T_Weapon.T_Weapon"))
  (return (`|GetArrayItem` _outrownames (`KismetMathLibrary.RandomInteger` (`KismetArrayLibrary.Array_Length` _outrownames)))))

(fn `Is Random Weapon?`
  (returns (NewParam :type Boolean))
  (bind _returnvalue (`DataTableFunctionLibrary.DoesDataTableRowExist` "/Game/ShootingGame/Data/T_Weapon.T_Weapon" (`self.WeaponName`)))
  (if _returnvalue
    (return false)
    (else
      (return true))))

(fn `Spawn Actor`
  (bind (_returnvalue_location _returnvalue_rotation _returnvalue_scale) (`KismetMathLibrary.BreakTransform` (`self.GetTransform`)))
  (bind (_returnvalue_x _returnvalue_y _returnvalue_z) (`KismetMathLibrary.BreakVector` (`self.K2_GetActorLocation`)))
  (`/Engine/EditorBlueprintResources/ActorMacros.Switch Has Authority`
    (:`Authority`
      (bind _randomlocation (`NavigationSystemV1.K2_GetRandomLocationInNavigableRadius` (`KismetMathLibrary.MakeVector` _returnvalue_x _returnvalue_y _returnvalue_z) 7000.0 null null))
      (bind (_outhit _returnvalue) (`KismetSystemLibrary.LineTraceSingleForObjects` :`Start` _randomlocation :`End` (`KismetMathLibrary.MakeVector` (.x _randomlocation) (.y _randomlocation) -100000.0) :`ObjectTypes` (`|MakeArray` "ObjectTypeQuery1" :!type "EObjectTypeQuery Enum") :`DrawDebugType` "ForDuration"))
      (if _returnvalue
        (bind _returnvalue_2 (`|GetDataTableRow` "/Game/ShootingGame/Data/T_Weapon.T_Weapon" (`self.Get Random Weapon Name`))
          (:`then`
            (`KismetSystemLibrary.PrintString` "Hello" false false)
            (bind (_weaponclass _staticmesh _maxammo _damage) (break `/Game/ShootingGame/Data/ST_Weapon` _returnvalue_2))
            (bind _returnvalue_3 (`|SpawnActorFromClass` _weaponclass (`KismetMathLibrary.MakeTransform` (`KismetMathLibrary.MakeVector` (.x (`.Location` (`GameplayStatics.BreakHitResult` _outhit))) (.y (`.Location` (`GameplayStatics.BreakHitResult` _outhit))) (+ (.z (`.Location` (`GameplayStatics.BreakHitResult` _outhit))) 100.0)) _returnvalue_rotation _returnvalue_scale) "AdjustIfPossibleButAlwaysSpawn" "OverrideRootScale" null (make `/Game/ShootingGame/Data/ST_Weapon` null _staticmesh _maxammo _damage) null))
            (set `self.Weapon` _returnvalue_3)))))))

(fn `UserConstructionScript`)