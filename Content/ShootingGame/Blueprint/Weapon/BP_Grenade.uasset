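; Thrown grenade that launches on BeginPlay with its Velocity and, given a valid OwnCharacter, explodes after a fixed fuse.
; Detonation plays sound and particles, fires a radial force impulse, and damages destructible components found by a debug-drawn sphere trace.
; It then applies falloff radial damage credited to the owner's controller, hides the mesh and sets a short lifespan for cleanup.
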(event `self.ReceiveBeginPlay`
  (`self.Throw` (`self.Velocity`)))

(event `Throw`
  (params (Velocity :type "Vector Structure"))
  (bind _returnvalue (`self.K2_GetActorLocation`))
  (bind _projectilemovement (`self.ProjectileMovement`))
  (set `MovementComponent.Velocity` Velocity _projectilemovement)
  (`ActorComponent.Activate` _projectilemovement false)
  (`/Engine/EditorBlueprintResources/StandardMacros.IsValid` (`self.Own Character`)
    (:`Is Valid`
      (`KismetSystemLibrary.Delay` 1.5)
      (`self.Show effet`)
      (`RadialForceComponent.FireImpulse` (`self.RadialForce`))
      (`|ExecutionSequence`
        (:`then_0`
          (bind _outhits (`KismetSystemLibrary.SphereTraceMultiForObjects` :`Start` _returnvalue :`End` _returnvalue :`Radius` 500.0 :`ObjectTypes` (`|MakeArray` "ObjectTypeQuery6" :!type "EObjectTypeQuery Enum") :`DrawDebugType` "ForDuration"))
          (for _array_element _outhits
            (bind _asdestructible_component (cast `DestructibleComponent` (`.HitComponent` (`GameplayStatics.BreakHitResult` _array_element))))
            (`self.Res Destructible Damage` _asdestructible_component (`SceneComponent.K2_GetComponentLocation` _asdestructible_component))))
        (:`then_1`
          (`GameplayStatics.ApplyRadialDamageWithFalloff` :`BaseDamage` 100.0 :`MinimumDamage` 30.0 :`Origin` (`self.K2_GetActorLocation`) :`DamageInnerRadius` 50.0 :`DamageOuterRadius` 500.0 :`DamageFalloff` 2.0 :`DamageTypeClass` "/Script/Engine.DamageType" :`DamageCauser` self :`InstigatedByController` (`Pawn.GetController` (`self.Own Character`)))
          (`SceneComponent.SetHiddenInGame` (`self.StaticMesh`) true false)
          (`self.SetLifeSpan` 3.0))))))

(event `Res Destructible Damage`
  (params (`Destructible Component` :type "DestructibleComponent Object Reference") (Origin :type "Vector Structure"))
  (`DestructibleComponent.ApplyRadiusDamage` `Destructible Component` 100.0 Origin 500.0 2000.0 false))

(event `Show effet`
  (bind _returnvalue (`SceneComponent.K2_GetComponentLocation` (`self.StaticMesh`)))
  (`GameplayStatics.PlaySoundAtLocation` "/Game/MilitaryWeapDark/Sound/GrenadeLauncher/GrenadeLauncher_Explosion_Cue.GrenadeLauncher_Explosion_Cue" _returnvalue (struct) 1.0 1.0 0.0 null null null)
  (`GameplayStatics.SpawnEmitterAtLocation` "/Game/MilitaryWeapDark/FX/P_Grenade_Explosion_01.P_Grenade_Explosion_01" _returnvalue))

(fn `UserConstructionScript`)