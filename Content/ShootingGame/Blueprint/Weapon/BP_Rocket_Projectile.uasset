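; BP_Rocket_Projectile is a rocket projectile that explodes when its box overlaps any actor other than its owning character.
; It activates its ProjectileMovement on BeginPlay, and on impact plays explosion sound and particles and fires a radial force impulse.
; A sphere trace then applies radius damage to nearby destructible components, with debug drawing left on.
; Finally it deals radial damage with falloff, credited to the owner's controller, and destroys itself.
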(event `self.ReceiveBeginPlay`
  (`ActorComponent.Activate` (`self.ProjectileMovement`) false))

(event `self.ReceiveTick`
  (params (DeltaSeconds :type "Float (single-precision)")))

(event `Res Destructible Damage`
  (params (`Destructible Component` :type "DestructibleComponent Object Reference") (Origin :type "Vector Structure"))
  (`DestructibleComponent.ApplyRadiusDamage` `Destructible Component` 1000.0 Origin 800.0 5000.0 true))

(event `self.Box.OnComponentBeginOverlap`
  (params (OverlappedComponent :type "PrimitiveComponent Object Reference") (OtherActor :type "Actor Object Reference") (OtherComp :type "PrimitiveComponent Object Reference") (OtherBodyIndex :type Integer) (bFromSweep :type Boolean) (SweepResult :type "HitResult Structure (by ref)"))
  (bind _returnvalue (`self.K2_GetActorLocation`))
  (if (!= OtherActor (`self.OwnerCharacter`))
    (`self.Res Shoot`)
    (`|ExecutionSequence`
      (:`then_0`
        (bind _outhits (`KismetSystemLibrary.SphereTraceMultiForObjects` :`Start` _returnvalue :`End` _returnvalue :`Radius` 800.0 :`ObjectTypes` (`|MakeArray` "ObjectTypeQuery6" :!type "EObjectTypeQuery Enum") :`DrawDebugType` "ForDuration"))
        (for _array_element _outhits
          (bind _asdestructible_component (cast `DestructibleComponent` (`.HitComponent` (`GameplayStatics.BreakHitResult` _array_element))))
          (`self.Res Destructible Damage` _asdestructible_component (`SceneComponent.K2_GetComponentLocation` _asdestructible_component))))
      (:`then_1`
        (`GameplayStatics.ApplyRadialDamageWithFalloff` :`BaseDamage` 250.0 :`MinimumDamage` 50.0 :`Origin` (`self.K2_GetActorLocation`) :`DamageInnerRadius` 50.0 :`DamageOuterRadius` 800.0 :`DamageFalloff` 2.0 :`DamageTypeClass` "/Script/Engine.DamageType" :`DamageCauser` self :`InstigatedByController` (`Pawn.GetController` (`self.OwnerCharacter`)))
        (`self.K2_DestroyActor`)))))

(event `Res Shoot`
  (`GameplayStatics.PlaySoundAtLocation` "/Game/MilitaryWeapDark/Sound/RocketLauncher/RocketLauncher_Explosion_Cue.RocketLauncher_Explosion_Cue" (`SceneComponent.K2_GetComponentLocation` (`self.StaticMesh`)) (struct) 1.0 1.0 0.0 null null null)
  (`GameplayStatics.SpawnEmitterAtLocation` "/Game/MilitaryWeapDark/FX/P_RocketLauncher_Explosion_01.P_RocketLauncher_Explosion_01" (`self.K2_GetActorLocation`))
  (`RadialForceComponent.FireImpulse` (`self.RadialForce`)))

(fn `UserConstructionScript`)