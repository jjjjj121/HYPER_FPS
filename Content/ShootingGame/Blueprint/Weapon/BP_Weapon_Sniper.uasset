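; Sniper rifle weapon for a networked shooter, overriding parent weapon behavior for firing and scoped aiming.
; Firing plays muzzle effects and sound, while the owning player shakes the camera and requests a hit check from the muzzle when zoomed, otherwise the camera.
; The server hit check consumes ammo, line-traces, and damages actors and destructibles.
; Aiming blends the view to the weapon, swaps in the scope HUD, and supports clamped FOV zoom.
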(event `self.ReceiveBeginPlay`
  (`parent.ReceiveBeginPlay`))

(fn `EventNotifyFire`
  (params (character :type "Character Object Reference"))
  (bind _returnvalue (`GameplayStatics.GetPlayerCameraManager` 0))
  (bind _staticmesh (`self.StaticMesh`))
  (`/Engine/EditorBlueprintResources/ActorMacros.Switch Has Authority`
    (:`Authority`
      (if (`self.Can Use Ammo`)
        (`GameplayStatics.SpawnEmitterAttached` (`self.Spawn Emitter`) _staticmesh "muzzle" (`SceneComponent.GetSocketLocation` _staticmesh "muzzle") (`SceneComponent.GetSocketRotation` _staticmesh "muzzle") (1.0 1.0 1.0) "KeepWorldPosition" :!label _label)
        (`AudioComponent.Play` (`self.Shoot Audio`) 0.0)
        (`self.Check My Owner`
          (:`True`
            (`self.ShakeCamera`)
            (`KismetSystemLibrary.PrintString` "EventNotifyFire" false false)
            (if (`/Game/ShootingGame/GameMode/BP_HyperCharacter.Is Zoom?` (`self.Own Character`))
              (`self.ReqHitCheck` (`SceneComponent.GetSocketLocation` (`self.StaticMesh`) "muzzle") (`self.GetActorForwardVector` (`GameplayStatics.GetPlayerCameraManager` 0)))
              (else
                (`self.ReqHitCheck` (`PlayerCameraManager.GetCameraLocation` _returnvalue) (`self.GetActorForwardVector` _returnvalue))))))))
    (:`Remote`
      (bind _isusedammo (`self.Use Ammo`))
      (if _isusedammo
        (goto _label)))))

(fn `Release Trigger`)

(fn `Server Hit Check`
  (params (Location :type "Vector Structure") (`Forward Vector` :type "Vector Structure"))
  (bind (_weaponref_weaponclass _weaponref_staticmesh _weaponref_maxammo _weaponref_damage) (break `/Game/ShootingGame/Data/ST_Weapon` (`self.WeaponRef`)))
  (bind (_weaponref_weaponclass_2 _weaponref_staticmesh_2 _weaponref_maxammo_2 _weaponref_damage_2) (break `/Game/ShootingGame/Data/ST_Weapon` (`self.WeaponRef`)))
  (bind _isusedammo (`self.Use Ammo`))
  (if _isusedammo
    (bind _outhit (`KismetSystemLibrary.LineTraceSingleForObjects` :`Start` (+ Location (* `Forward Vector` 1.0)) :`End` (+ Location (* `Forward Vector` 10000.0)) :`ObjectTypes` (`|MakeArray` "ObjectTypeQuery1" "ObjectTypeQuery2" "ObjectTypeQuery3" "ObjectTypeQuery4" "ObjectTypeQuery5" "ObjectTypeQuery6" :!type "EObjectTypeQuery Enum") :`DrawDebugType` "ForDuration"))
    (bind (_bblockinghit _binitialoverlap _time _distance _location _impactpoint _normal _impactnormal _physmat _hitactor _hitcomponent _hitbonename _hititem _elementindex _faceindex _tracestart _traceend) (`GameplayStatics.BreakHitResult` _outhit))
    (`GameplayStatics.SpawnEmitterAtLocation` "/Game/MilitaryWeapDark/FX/P_Impact_Metal_Medium_01.P_Impact_Metal_Medium_01" _location)
    (`|ExecutionSequence`
      (:`then_0`
        (`GameplayStatics.ApplyDamage` _hitactor _weaponref_damage_2 (`Pawn.GetController` (`self.Own Character`)) self) ; 번개표시 = 서버에서만 실행
        (`self.ResImpactEffect` _impactpoint))
      (:`then_1`
        (bind _asdestructible_component (cast `DestructibleComponent` _hitcomponent))
        (`self.Destructible Damage` _asdestructible_component _weaponref_damage _location _impactpoint)))))

(fn `ShakeCamera`
  (`PlayerController.ClientStartCameraShake` :`self` (`GameplayStatics.GetPlayerController` 0) :`Shake` "/Game/ShootingGame/ShootShakeCamera_Sniper.ShootShakeCamera_Sniper_C" :`Scale` (`self.Shake Camera Scale`)))

(fn `Toggle Aim`
  (params (Character :type "/Game/ShootingGame/GameMode/BP_HyperCharacter Object Reference") (`Is Press?` :type Boolean))
  (returns (`Toggle Aim` :type Boolean))
  (bind _shooting_hud (`/Game/ShootingGame/GameMode/BP_HyperCharacter.Shooting HUD` Character))
  (bind _aim (`/Game/ShootingGame/GameMode/BP_ShootingHUD.Aim` _shooting_hud))
  (bind _sniper_aim (`/Game/ShootingGame/GameMode/BP_ShootingHUD.Sniper Aim` _shooting_hud))
  (if `Is Press?`
    (`PlayerCameraManager.StartCameraFade` :`self` (`PlayerController.PlayerCameraManager` (`GameplayStatics.GetPlayerController` 0)) :`FromAlpha` 1.0 :`Duration` 2.0)
    (`PlayerController.SetViewTargetWithBlend` (`GameplayStatics.GetPlayerController` 0) self 0.3 "VTBlend_Linear" 0.0 false)
    (`Widget.SetVisibility` _sniper_aim "Visible")
    (`Widget.SetVisibility` _aim "Collapsed")
    (return true)
    (else
      (`PlayerController.SetViewTargetWithBlend` (`GameplayStatics.GetPlayerController` 0) Character 0.3 "VTBlend_Linear" 0.0 false)
      (`Widget.SetVisibility` _sniper_aim "Collapsed")
      (`Widget.SetVisibility` _aim "Visible")
      (return false))))

(fn `UserConstructionScript`
  (`parent.UserConstructionScript`))

(fn `Zoom`
  (params (`delta value` :type "Float (double-precision)") (`Zoom In?` :type Boolean))
  (returns (NewParam1 :type Boolean))
  (bind _returnvalue (* `delta value` (`GameplayStatics.GetWorldDeltaSeconds`)))
  (bind _fieldofview (`CameraComponent.FieldOfView` (`self.Camera`)))
  (if `Zoom In?`
    (`CameraComponent.SetFieldOfView` (`self.Camera`) (`KismetMathLibrary.FClamp` (+ (* _returnvalue -1.0) _fieldofview) 10.0 45.0))
    (else
      (`CameraComponent.SetFieldOfView` (`self.Camera`) (`KismetMathLibrary.FClamp` (+ _returnvalue _fieldofview) 10.0 45.0)))))