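; Grenade launcher weapon that shows an aiming arc while the trigger is held and fires BP_Grenade on release.
; For the owning player, ShowSpline re-runs on a per-frame timer, turning the predicted projectile path into spline meshes and a landing decal.
; Release plays the fire montage; EventNotifyFire adds effects and requests ServerHitCheck, which consumes ammo and spawns the grenade.
; Detaching clears the preview and enables weapon physics.
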(event `self.ReqHitCheck`
  (params (Location :type "Vector Structure") (`Forward Vector` :type "Vector Structure"))
  (`self.Server Hit Check` Location `Forward Vector`))

(event `Req Hit Check2`
  (params (Location :type "Vector Structure") (`Forward Vector` :type "Vector Structure"))
  (`self.Server Hit Check` Location `Forward Vector`))

(fn `DetachToCharacter`
  (params (Character :type "Character Object Reference"))
  (bind _staticmesh (`self.StaticMesh`))
  (bind _spline_meshes (`self.Spline Meshes`))
  (`SplineComponent.ClearSplinePoints` (`self.Spline`) true)
  (`ActorComponent.K2_DestroyComponent` _spline_meshes)
  (`KismetArrayLibrary.Array_Clear` _spline_meshes)
  (`SceneComponent.SetVisibility` (`self.Hit Decal`) false false)
  (`PrimitiveComponent.SetCollisionEnabled` _staticmesh "QueryAndPhysics")
  (`PrimitiveComponent.SetSimulatePhysics` _staticmesh true)
  (`self.Update UI` 0)
  ;[1 1 1] UnEquip 상태로 정보 변경
  (bind _asbp_hyper_character (cast `/Game/ShootingGame/GameMode/BP_HyperCharacter` Character))
  (set `/Game/ShootingGame/GameMode/BP_HyperCharacter.Attached Weapon` null _asbp_hyper_character)
  (set `self.Own Character` null)
  (set `Pawn.bUseControllerRotationYaw` false _asbp_hyper_character)
  (set `CharacterMovementComponent.bOrientRotationToMovement` true (`Character.CharacterMovement` _asbp_hyper_character))
  (if (`/Game/ShootingGame/GameMode/BP_HyperCharacter.Is Death` _asbp_hyper_character)
    (`self.K2_DetachFromActor` "KeepWorld" "KeepWorld" "KeepWorld")))

(fn `EventNotifyFire`
  (params (character :type "Character Object Reference"))
  (bind _staticmesh (`self.StaticMesh`))
  ;[1 1 1] Client
  (`/Engine/EditorBlueprintResources/ActorMacros.Switch Has Authority`
    (:`Authority`
      (if (`self.Can Use Ammo`)
        (`GameplayStatics.SpawnEmitterAttached` (`self.Spawn Emitter`) _staticmesh "muzzle" (`SceneComponent.GetSocketLocation` _staticmesh "muzzle") (`SceneComponent.GetSocketRotation` _staticmesh "muzzle") (1.0 1.0 1.0) "KeepWorldPosition" :!label _label)
        (`AudioComponent.Play` (`self.Shoot Audio`) 0.0)
        (`self.Check My Owner`
          (:`True`
            (`self.ShakeCamera`)
            (`KismetSystemLibrary.PrintString` "EventNotifyFire" false false)
            (`self.Req Hit Check2` (`SceneComponent.GetSocketLocation` (`self.StaticMesh`) "muzzle") (* (`KismetMathLibrary.GetForwardVector` (`Pawn.GetControlRotation` (`self.Own Character`))) 3000.0))))))
    (:`Remote`
      (bind _isusedammo (`self.Use Ammo`))
      (if _isusedammo
        (goto _label)))))

(fn `PullTrigger`
  (params (Character :type "Character Object Reference"))
  (`self.Check My Owner`
    (:`True`
      (set `self.throwing` true)
      (`self.Show Spline`))))

(fn `Release Trigger`
  (set `self.throwing` false)
  (`SceneComponent.SetVisibility` (`self.Hit Decal`) false false)
  (`Character.PlayAnimMontage` (`self.Own Character`) "/Game/ShootingGame/Animation/My_Fire_Reload_Equip_Jump/AM_Rifle_Fire.AM_Rifle_Fire" 1.0 "None")
  (set `self.Recoil Vector` (* (`self.GetActorForwardVector` (`GameplayStatics.GetPlayerCameraManager` 0)) 100000.0)))

(fn `Server Hit Check`
  (params (Location :type "Vector Structure") (`Forward Vector` :type "Vector Structure"))
  (bind _own_character (`self.Own Character`))
  (bind _isusedammo (`self.Use Ammo`))
  (if _isusedammo
    (`|SpawnActorFromClass` "/Game/ShootingGame/Blueprint/Weapon/BP_Grenade.BP_Grenade_C" (`KismetMathLibrary.MakeTransform` Location (`SceneComponent.GetSocketRotation` (`self.StaticMesh`) "muzzle") (5.0 5.0 5.0)) "AlwaysSpawn" "OverrideRootScale" _own_character _own_character `Forward Vector` null)))

(fn `Show Spline`
  (bind _hit_decal (`self.Hit Decal`))
  (bind _spline (`self.Spline`))
  (bind _spline_2 (`self.Spline`))
  (bind _spline_meshes (`self.Spline Meshes`))
  (`/Engine/EditorBlueprintResources/StandardMacros.IsValid` (`self.Own Character`)
    (:`Is Valid`
      (`SplineComponent.ClearSplinePoints` (`self.Spline`) true)
      (`ActorComponent.K2_DestroyComponent` _spline_meshes)
      (`KismetArrayLibrary.Array_Clear` _spline_meshes)
      (if (`self.throwing`)
        (bind (_outhit _outpathpositions _outlasttracedestination) (`GameplayStatics.Blueprint_PredictProjectilePath_ByObjectType` :`StartPos` (`SceneComponent.GetSocketLocation` (`self.StaticMesh`) "muzzle") :`LaunchVelocity` (* (`KismetMathLibrary.GetForwardVector` (`Pawn.GetControlRotation` (`self.Own Character`))) 3000.0) :`ObjectTypes` (`|MakeArray` "ObjectTypeQuery1" "ObjectTypeQuery2" "ObjectTypeQuery3" "ObjectTypeQuery4" "ObjectTypeQuery5" :!type "EObjectTypeQuery Enum") :`DrawDebugTime` 3.0))
        (`SceneComponent.K2_SetWorldLocationAndRotation` :`self` _hit_decal :`NewLocation` _outlasttracedestination)
        (`SceneComponent.SetVisibility` _hit_decal true false)
        (for (_array_element _array_index) _outpathpositions
          (`SplineComponent.AddSplinePointAtIndex` _spline_2 _array_element _array_index "Local" true))
        (for _index (range (+ (- (`SplineComponent.GetNumberOfSplinePoints` _spline_2) 2) 1))
          (bind _returnvalue (`AddComponent|NODE_AddSplineMeshComponent-2` :`bManualAttachment` true :`RelativeTransform` (`KismetMathLibrary.MakeTransform` (0.0 0.0 0.0))))
          (`KismetArrayLibrary.Array_Add` (`self.Spline Meshes`) _returnvalue)
          (bind _returnvalue_2 (+ _index 1))
          (`SplineMeshComponent.SetStartAndEnd` _returnvalue (`SplineComponent.GetLocationAtSplinePoint` _spline _index "Local") (`SplineComponent.GetTangentAtSplinePoint` _spline _index "Local") (`SplineComponent.GetLocationAtSplinePoint` _spline _returnvalue_2 "Local") (`SplineComponent.GetTangentAtSplinePoint` _spline _returnvalue_2 "Local") true))
        (if (`self.throwing`)
          (`KismetSystemLibrary.K2_SetTimer` null "Show Spline" (`GameplayStatics.GetWorldDeltaSeconds`)))))))

(fn `UserConstructionScript`
  (`parent.UserConstructionScript`))