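; Rocket launcher weapon Blueprint for a networked shooter, overriding its parent's fire, trigger and reload logic with a small magazine.
; The fire notify plays muzzle effects, audio and a loading montage, and blocks the trigger until the reload-end notify.
; Only the owning player shakes the camera and sends its camera aim through ReqHitCheck.
; ServerHitCheck consumes ammo and spawns the rocket projectile along the muzzle socket's rotation.
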(event `self.ReceiveBeginPlay`
  (`StaticMeshComponent.SetStaticMesh` (`self.StaticMesh`) "/Game/MilitaryWeapDark/Weapons/Mesh/StaticMesh_Rocket_Launcher.StaticMesh_Rocket_Launcher")
  (set `self.Ammo` 3))

(event `self.ReqHitCheck`
  (params (Location :type "Vector Structure") (`Forward Vector` :type "Vector Structure"))
  (`parent.ReqHitCheck` Location `Forward Vector`))

(fn `EventNotify End Reload`
  (set `self.Is Running?` false))

(fn `EventNotifyFire`
  (params (character :type "Character Object Reference"))
  (bind _returnvalue (`GameplayStatics.GetPlayerCameraManager` 0))
  (bind _staticmesh (`self.StaticMesh`))
  ;[1 1 1] Client
  (set `self.Is Running?` true)
  (`/Engine/EditorBlueprintResources/ActorMacros.Switch Has Authority`
    (:`Authority`
      (if (`self.Can Use Ammo`)
        (`GameplayStatics.SpawnEmitterAttached` (`self.Spawn Emitter`) _staticmesh "muzzle" (`SceneComponent.GetSocketLocation` _staticmesh "muzzle") (`SceneComponent.GetSocketRotation` _staticmesh "muzzle") (1.0 1.0 1.0) "KeepWorldPosition" :!label _label)
        (`AudioComponent.Play` (`self.Shoot Audio`) 0.0)
        (`Character.PlayAnimMontage` (`self.Own Character`) "/Game/RifleAnimsetPro/Animations/Rocket_Loading_Reload_Montage.Rocket_Loading_Reload_Montage" 1.0 "None")
        (`self.Check My Owner`
          (:`True`
            (`self.ShakeCamera`)
            (`KismetSystemLibrary.PrintString` "EventNotifyFire" false false)
            (`self.ReqHitCheck` (`self.K2_GetActorLocation` _returnvalue) (`self.GetActorForwardVector` _returnvalue))))))
    (:`Remote`
      (bind _isusedammo (`self.Use Ammo`))
      (if _isusedammo
        (goto _label)))))

(fn `PullTrigger`
  (params (Character :type "Character Object Reference"))
  (if (`self.Is Running?`)
    _
    (elif (`self.Can Use Ammo`)
      (`Character.PlayAnimMontage` (`self.Own Character`) "/Game/ShootingGame/Animation/My_Fire_Reload_Equip_Jump/AM_Rifle_Fire.AM_Rifle_Fire" 1.0 "None")
      (set `self.Recoil Vector` (* (`self.GetActorForwardVector` (`GameplayStatics.GetPlayerCameraManager` 0)) 100000.0)))))

(fn `Reload`
  (if (and (< (`self.Ammo`) 3) (`/Game/ShootingGame/GameMode/BP_HyperCharacter.Has Mag` (`self.Own Character`)))
    (`Character.PlayAnimMontage` (`self.Own Character`) "/Game/ShootingGame/Animation/My_Fire_Reload_Equip_Jump/AS_Rifle_ReloadLoaded_Montage.AS_Rifle_ReloadLoaded_Montage" 1.0 "None")))

(fn `Server Hit Check`
  (params (Location :type "Vector Structure") (`Forward Vector` :type "Vector Structure"))
  (bind _staticmesh (`self.StaticMesh`))
  (bind _own_character (`self.Own Character`))
  (bind _isusedammo (`self.Use Ammo`))
  (if _isusedammo
    (`|SpawnActorFromClass` "/Game/ShootingGame/Blueprint/Weapon/BP_Rocket_Projectile.BP_Rocket_Projectile_C" (`KismetMathLibrary.MakeTransform` (`SceneComponent.GetSocketLocation` _staticmesh "muzzle") (`SceneComponent.GetSocketRotation` _staticmesh "muzzle")) "AlwaysSpawn" "OverrideRootScale" _own_character _own_character null)))

(fn `Set Ammo`
  (bind _is_used_mag (`/Game/ShootingGame/GameMode/BP_HyperCharacter.UseMag` (`self.Own Character`)))
  (if _is_used_mag
    (bind _output_get (set `self.Ammo` 3))
    (`self.Update UI` _output_get)))

(fn `ShakeCamera`
  (`PlayerController.ClientStartCameraShake` :`self` (`GameplayStatics.GetPlayerController` 0) :`Shake` "/Game/ShootingGame/ShootShakeCamera_RocketLauncher.ShootShakeCamera_RocketLauncher_C" :`Scale` (`self.Shake Camera Scale`)))

(fn `UserConstructionScript`
  (`parent.UserConstructionScript`))