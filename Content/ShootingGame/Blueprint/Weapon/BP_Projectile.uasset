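; BP_Projectile is a rocket-style projectile that explodes on overlap and deals radial damage.
; Tick pushes its skeletal mesh along the actor's forward vector at constant speed without sweeping.
; A Box overlap with anything but the owner character spawns an explosion emitter, fires a radial impulse and applies falloff damage credited to the owner's controller, drawing debug spheres for both radii.
; The projectile never destroys itself, and an authority switch is left unconnected.
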(event `self.ReceiveBeginPlay`
  (`KismetSystemLibrary.PrintString` "projectile Create" false false (struct :`G` 0.66 :`B` 1.0 :`A` 1.0) 60.0))

(event `self.ReceiveTick`
  (params (DeltaSeconds :type "Float (single-precision)"))
  (`SceneComponent.K2_AddWorldOffset` (`self.SkeletalMesh`) (* (* (`self.GetActorForwardVector`) DeltaSeconds) 5000.0) false false))

(event `self.Box.OnComponentBeginOverlap`
  (params (OverlappedComponent :type "PrimitiveComponent Object Reference") (OtherActor :type "Actor Object Reference") (OtherComp :type "PrimitiveComponent Object Reference") (OtherBodyIndex :type Integer) (bFromSweep :type Boolean) (SweepResult :type "HitResult Structure (by ref)"))
  (bind _returnvalue (`self.K2_GetActorLocation`))
  (if (!= OtherActor (`self.OwnerCharacter`))
    (`GameplayStatics.SpawnEmitterAtLocation` "/Game/MilitaryWeapDark/FX/P_RocketLauncher_Explosion_01.P_RocketLauncher_Explosion_01" (`self.K2_GetActorLocation`))
    (`RadialForceComponent.FireImpulse` (`self.RadialForce`))
    (`GameplayStatics.ApplyRadialDamageWithFalloff` :`BaseDamage` 100.0 :`MinimumDamage` 50.0 :`Origin` _returnvalue :`DamageInnerRadius` 50.0 :`DamageOuterRadius` 500.0 :`DamageFalloff` 2.0 :`DamageTypeClass` "/Script/Engine.DamageType" :`DamageCauser` self :`InstigatedByController` (`Pawn.GetController` (`self.OwnerCharacter`)))
    (`KismetSystemLibrary.DrawDebugSphere` _returnvalue 50.0 24 (struct :`R` 1.0 :`G` 1.0 :`B` 1.0 :`A` 1.0) 2.0 1.0)
    (`KismetSystemLibrary.DrawDebugSphere` _returnvalue 500.0 24 (struct :`R` 1.0 :`G` 1.0 :`B` 1.0 :`A` 1.0) 2.0 1.0)))

(fn `UserConstructionScript`)