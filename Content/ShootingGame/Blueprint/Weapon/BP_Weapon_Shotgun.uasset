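; Shotgun weapon Blueprint that implements server-side hit checking for a multi-pellet spread shot.
; When ammo is consumed, it fires five debug-drawn line traces in a random elliptical cone, starting nearer the given location when the owner is zoomed.
; Each trace spawns an impact particle, applies WeaponRef damage, calls ResImpactEffect (handled by the parent) and damages any destructible component hit.
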(event `self.ResImpactEffect`
  (params (`Impact Loaction` :type "Vector Structure"))
  (`parent.ResImpactEffect` `Impact Loaction`))

(fn `Server Hit Check`
  (params (Location :type "Vector Structure") (`Forward Vector` :type "Vector Structure"))
  (bind (_weaponref_weaponclass _weaponref_staticmesh _weaponref_maxammo _weaponref_damage) (break `/Game/ShootingGame/Data/ST_Weapon` (`self.WeaponRef`)))
  (bind (_weaponref_weaponclass_2 _weaponref_staticmesh_2 _weaponref_maxammo_2 _weaponref_damage_2) (break `/Game/ShootingGame/Data/ST_Weapon` (`self.WeaponRef`)))
  (bind (_weaponref_weaponclass_3 _weaponref_staticmesh_3 _weaponref_maxammo_3 _weaponref_damage_3) (break `/Game/ShootingGame/Data/ST_Weapon` (`self.WeaponRef`)))
  (bind (_weaponref_weaponclass_4 _weaponref_staticmesh_4 _weaponref_maxammo_4 _weaponref_damage_4) (break `/Game/ShootingGame/Data/ST_Weapon` (`self.WeaponRef`)))
  (bind _isusedammo (`self.Use Ammo`))
  (if _isusedammo
    (if (`/Game/ShootingGame/GameMode/BP_HyperCharacter.Is Zoom?` (`self.Own Character`))
      (for _ (range 1 6)
        (bind _outhit (`KismetSystemLibrary.LineTraceSingleForObjects` :`Start` (+ Location (* `Forward Vector` 100.0)) :`End` (+ Location (* (`KismetMathLibrary.RandomUnitVectorInEllipticalConeInDegrees` `Forward Vector` 15.0 5.0) 10000.0)) :`ObjectTypes` (`|MakeArray` "ObjectTypeQuery1" "ObjectTypeQuery2" "ObjectTypeQuery3" "ObjectTypeQuery4" "ObjectTypeQuery5" "ObjectTypeQuery6" :!type "EObjectTypeQuery Enum") :`DrawDebugType` "ForDuration"))
        (bind (_bblockinghit _binitialoverlap _time _distance _location _impactpoint _normal _impactnormal _physmat _hitactor _hitcomponent) (`GameplayStatics.BreakHitResult` _outhit))
        (`GameplayStatics.SpawnEmitterAtLocation` "/Game/MilitaryWeapDark/FX/P_Impact_Metal_Medium_01.P_Impact_Metal_Medium_01" _location)
        (`|ExecutionSequence`
          (:`then_0`
            (`GameplayStatics.ApplyDamage` _hitactor _weaponref_damage_2 (`Pawn.GetController` (`self.Own Character`)) self) ; 번개표시 = 서버에서만 실행
            (`self.ResImpactEffect` _location))
          (:`then_1`
            (bind _asdestructible_component (cast `DestructibleComponent` _hitcomponent))
            (`self.Destructible Damage` _asdestructible_component _weaponref_damage_4 _location _impactpoint))))
      (else
        (for _ (range 1 6)
          (bind _outhit_2 (`KismetSystemLibrary.LineTraceSingleForObjects` :`Start` (+ Location (* `Forward Vector` 380.0)) :`End` (+ Location (* (`KismetMathLibrary.RandomUnitVectorInEllipticalConeInDegrees` `Forward Vector` 15.0 5.0) 10000.0)) :`ObjectTypes` (`|MakeArray` "ObjectTypeQuery1" "ObjectTypeQuery2" "ObjectTypeQuery3" "ObjectTypeQuery4" "ObjectTypeQuery5" "ObjectTypeQuery6" :!type "EObjectTypeQuery Enum") :`DrawDebugType` "ForDuration"))
          (bind (_bblockinghit_2 _binitialoverlap_2 _time_2 _distance_2 _location_2 _impactpoint_2 _normal_2 _impactnormal_2 _physmat_2 _hitactor_2 _hitcomponent_2) (`GameplayStatics.BreakHitResult` _outhit_2))
          (`GameplayStatics.SpawnEmitterAtLocation` "/Game/MilitaryWeapDark/FX/P_Impact_Metal_Medium_01.P_Impact_Metal_Medium_01" _location_2)
          (`|ExecutionSequence`
            (:`then_0`
              (`GameplayStatics.ApplyDamage` _hitactor_2 _weaponref_damage_3 (`Pawn.GetController` (`self.Own Character`)) self) ; 번개표시 = 서버에서만 실행
              (`self.ResImpactEffect` _location_2))
            (:`then_1`
              (bind _asdestructible_component_2 (cast `DestructibleComponent` _hitcomponent_2))
              (`self.Destructible Damage` _asdestructible_component_2 _weaponref_damage _location_2 _impactpoint_2))))))))

(fn `UserConstructionScript`
  (`parent.UserConstructionScript`))