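; Burst-fire weapon Blueprint that overrides the trigger and repeat-shot logic of its parent weapon class.
; PullTrigger runs the parent logic, then sets a small fixed count of follow-up shots.
; AddShoot replaces the parent version, playing the rifle fire montage on the owning character and decrementing the count per call.
; Once the count runs out, it clears the AddShoot timer, which is not started in this Blueprint.
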(fn `AddShoot`
  (`/Engine/EditorBlueprintResources/StandardMacros.IsValid` (`self.Own Character`)
    (:`Is Valid`
      (if (> (`self.ShootCount`) 0)
        (`Character.PlayAnimMontage` (`self.Own Character`) "/Game/ShootingGame/Animation/My_Fire_Reload_Equip_Jump/AM_Rifle_Fire.AM_Rifle_Fire" 1.0 "None")
        (`/Engine/EditorBlueprintResources/StandardMacros.DecrementInt` (`self.ShootCount`))
        (else
          (`KismetSystemLibrary.K2_ClearTimer` null "AddShoot"))))))

(fn `PullTrigger`
  (params (Character :type "Character Object Reference"))
  (`parent.PullTrigger` Character)
  (set `self.ShootCount` 2))

(fn `UserConstructionScript`
  (`parent.UserConstructionScript`))