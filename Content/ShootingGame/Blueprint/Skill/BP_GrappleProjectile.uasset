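; Grappling-hook projectile that spins in flight and anchors itself to whatever it hits.
; Tick rotates the mesh through a gate, which closes on hit.
; A hit on another actor calls GrappleHit for the bound grappling component, disables collision, zeroes velocity, and attaches the hook at the impact point, aligned to the surface normal.
; A shared PlaySound helper swaps start, hit and delayed in-air sounds on one audio component.
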(event `self.ReceiveBeginPlay`
  (`self.PlaySound` (`self.StartingSound`) 0.25)
  (`KismetSystemLibrary.PrintString` "Hook Create" false false (struct :`G` 1.0 :`B` 0.135954 :`A` 1.0) 15.0)
  (`KismetSystemLibrary.PrintString` (`KismetStringLibrary.Concat_StrStr` "Compoenet : " (`KismetSystemLibrary.GetDisplayName` (`self.Hook`))) false false (struct :`G` 0.66 :`B` 1.0 :`A` 1.0) 15.0))

(event `self.ReceiveTick`
  (params (DeltaSeconds :type "Float (single-precision)"))
  (`/Engine/EditorBlueprintResources/StandardMacros.Gate` false :!label _label ; 벽에 닿았을 경우(Hit) 돌아가는 거 멈추게
    (:`Exit`
      (`SceneComponent.K2_AddLocalRotation` (`self.StaticMesh`) (`KismetMathLibrary.MakeRotator` 0.0 0.0 (* (`GameplayStatics.GetWorldDeltaSeconds`) 1000.0)) false false) ; 훅이 빙글빙글 돌면서 날아가게
    )))

(event `self.ReceiveHit`
  (params (MyComp :type "PrimitiveComponent Object Reference") (Other :type "Actor Object Reference") (OtherComp :type "PrimitiveComponent Object Reference") (bSelfMoved :type Boolean) (HitLocation :type "Vector Structure") (HitNormal :type "Vector Structure") (NormalImpulse :type "Vector Structure") (Hit :type "HitResult Structure (by ref)"))
  (bind (_bblockinghit _binitialoverlap _time _distance _location _impactpoint _normal _impactnormal _physmat _hitactor) (`GameplayStatics.BreakHitResult` Hit))
  (`|ExecutionSequence`
    (:`then_0`
      (goto _label :!via `Close`))
    (:`then_1`
      (if (!= self _hitactor)
        (`self.GrappleHit` Hit) ; Component에 바인딩 된\n그래플링 기능 호출
        (`PrimitiveComponent.SetCollisionEnabled` (`self.Collision`) "NoCollision")
        (`ProjectileMovementComponent.SetVelocityInLocalSpace` (`self.ProjectileMovement`) (0.0 0.0 0.0)) ; 닿은 위치에서 위치 고정하기 위해 속도값 0으로 Set
        (`self.K2_SetActorLocationAndRotation` _impactpoint (`KismetMathLibrary.MakeRotFromX` _impactnormal)) ; 히트된 위치에 훅 고정
        (`self.K2_AttachToActor` _hitactor "None" "KeepWorld" "KeepWorld" "KeepWorld")
        (`self.PlaySound` (`self.HitSound`))
        (`KismetSystemLibrary.Delay` 0.2)
        (`self.PlaySound` (`self.InAirSound`) 0.0 0.75)))))

(fn `PlaySound`
  (params (Sound :type "SoundBase Object Reference") (StartTime :type "Float (double-precision)") (PitchMultiplier :type "Float (double-precision)"))
  (bind _pitchmultiplier (`local.PitchMultiplier`))
  (bind _audio (`self.Audio`))
  (`AudioComponent.SetSound` _audio (`local.Sound`))
  (`AudioComponent.Play` _audio (`local.StartTime`))
  (if (!= _pitchmultiplier 0.0)
    (`AudioComponent.SetPitchMultiplier` (`self.Audio`) _pitchmultiplier)))

(fn `UserConstructionScript`)