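; Skill component for BP_HyperCharacter that gives a Tracer-style Q blink and E rewind.
; Q spends a SkillCount charge and teleports along a line trace, toward the supplied location when moving or straight forward when still, stopping at hits.
; Tick keeps a rolling 60-sample transform history, which E replays backwards through a delayed-loop macro, restoring control rotation only for the local player.
; When ECount runs out, the component requests server-side skill destruction.
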(event `Reverse`
  (`/Game/ShootingGame/GameMode/BP_HyperCharacter.Play E Trace Sound` (`self.Character`))
  ;[1 1 1] forloop delay 값씩 배열 0까지 되돌린다.
  (bind _element (`self.ReversedForLoop` (`self.Transform`) 0.008)
    (:`LoopBody`
      (`Actor.K2_SetActorLocation` (`self.Character`) (.location _element) false false)
      (`self.Check My Owner`
        (:`true`
          (`Controller.SetControlRotation` (`GameplayStatics.GetPlayerController` 0) (.rotation _element)))))
    (:`Completed`
      ;[1 1 1] 돌린수 배열 클리어
      (`KismetArrayLibrary.Array_Clear` (`self.Transform`))
      (set `self.E Count` (- (`self.E Count`) 1))
      (if (<= (`self.E Count`) 0)
        (set `/Game/ShootingGame/GameMode/BP_HyperCharacter.Skill Count` 0 (`self.Character`))
        (`/Game/ShootingGame/GameMode/BP_HyperCharacter.Update Skill Count` (`self.Character`) 0)
        (`self.Destroy Self`)))))

(event `self.ReceiveTick`
  (params (DeltaSeconds :type "Float (single-precision)"))
  (bind _transform (`self.Transform`))
  (if (<= (`self.E Count`) 0)
    (`self.Destroy Self`)
    (else
      (`self.AddLocation`)
      (if (> (`KismetArrayLibrary.Array_Length` _transform) 60)
        (`KismetArrayLibrary.Array_Remove` _transform)))))

(fn `AddLocation`
  (bind _character (`self.Character`))
  (`/Engine/EditorBlueprintResources/StandardMacros.IsValid` (`self.Character`)
    (:`Is Valid`
      (`KismetArrayLibrary.Array_Add` (`self.Transform`) (`KismetMathLibrary.MakeTransform` (`Actor.K2_GetActorLocation` _character) (`Pawn.GetControlRotation` _character))))))

(fn `CanTeleport`
  (returns (NewParam :type Boolean))
  (return (> (`self.Q Count`) 0)))

(fn `Client Press Q`
  (params (Character :type "Character Object Reference"))
  (returns (Result :type Boolean))
  (return false))

(fn `DecreaseCount`
  (set `self.Q Count` (- (`self.Q Count`) 1)))

(fn `Destroy Client Component`
  (returns (Result :type Boolean))
  (return false))

(fn `Destroy Self`
  (returns (Result :type Boolean))
  (`/Game/ShootingGame/GameMode/BP_HyperCharacter.Server Destroy Skill` (`self.Character`)))

(fn `Event Press E`
  (params (Character :type "Character Object Reference") (True :type Boolean))
  (returns (Result :type Boolean))
  (if (> (`self.E Count`) 0)
    (`self.Reverse`)))

(fn `EventPressQ`
  (params (Character :type "Character Object Reference") (Location :type "Vector Structure") (Rotation :type "Rotator Structure") (True :type Boolean))
  (returns (Result :type Boolean))
  (if (> (`/Game/ShootingGame/GameMode/BP_HyperCharacter.Skill Count` (`self.Character`)) 0)
    (set `self.Direction` Location)
    (if (<= (`/Game/ShootingGame/GameMode/BP_HyperCharacter.Skill Count` (`self.Character`)) 1)
      (`/Game/ShootingGame/GameMode/BP_HyperCharacter.Set Trace Count Zero` (`self.Character`))
      (else
        (`/Game/ShootingGame/GameMode/BP_HyperCharacter.Server Minus Skill Count` (`self.Character`))))
    (if (> (`KismetMathLibrary.VSize` (`Actor.GetVelocity` (`self.Character`))) 0.0)
      (`self.LineTraceMoving`)
      (else
        (`self.LinTraceStopMoving`)))
    (`/Game/ShootingGame/GameMode/BP_HyperCharacter.Play Q Trace Sound` (`self.Character`))))

(fn `FindLocation`
  (params (Transform :type "Transform Structure"))
  (returns (Result :type Boolean))
  (return false))

(fn `Get Value`
  (returns (Ratation :type "Rotator Structure") (Transform :type "Transform Structure"))
  (return))

(fn `Initialize`
  (params (Chracter :type "Character Object Reference") (`Skill Count` :type Integer))
  (returns (Result :type Boolean))
  (bind _asbp_hyper_character (cast `/Game/ShootingGame/GameMode/BP_HyperCharacter` Chracter))
  (set `self.Character` _asbp_hyper_character)
  (`/Game/ShootingGame/GameMode/BP_HyperCharacter.Update Skill Count Multi` (`self.Character`)))

(fn `LineTraceMoving`
  (bind _returnvalue (`Actor.K2_GetActorRotation` (`self.Character`)))
  (bind (_outhit _returnvalue_2) (`KismetSystemLibrary.LineTraceSingle` :`Start` (`Actor.K2_GetActorLocation` (`self.Character`)) :`End` (`self.Direction`) :`TraceChannel` "TraceTypeQuery1" :`DrawDebugType` "ForDuration"))
  (if _returnvalue_2
    (bind (_bblockinghit _binitialoverlap _time _distance _location _impactpoint _normal _impactnormal _physmat _hitactor _hitcomponent _hitbonename _hititem _elementindex _faceindex _tracestart _traceend) (`GameplayStatics.BreakHitResult` _outhit))
    (`Actor.K2_TeleportTo` (`self.Character`) _location _returnvalue)
    (else
      (`Actor.K2_TeleportTo` (`self.Character`) _traceend _returnvalue))))

(fn `LinTraceStopMoving`
  (bind _character (`self.Character`))
  (bind _returnvalue (`Actor.K2_GetActorLocation` _character))
  (bind (_outhit _returnvalue_2) (`KismetSystemLibrary.LineTraceSingle` :`Start` _returnvalue :`End` (+ (* (`Actor.GetActorForwardVector` _character) (`self.Range`)) _returnvalue) :`TraceChannel` "TraceTypeQuery1" :`DrawDebugType` "ForDuration"))
  (if _returnvalue_2
    (bind (_bblockinghit _binitialoverlap _time _distance _location _impactpoint _normal _impactnormal _physmat _hitactor _hitcomponent _hitbonename _hititem _elementindex _faceindex _tracestart _traceend) (`GameplayStatics.BreakHitResult` _outhit))
    (`Actor.K2_TeleportTo` (`self.Character`) _location (`Actor.K2_GetActorRotation` (`self.Character`)))
    (else
      (`Actor.K2_TeleportTo` (`self.Character`) _traceend (`Actor.K2_GetActorRotation` (`self.Character`))))))

(fn `Server Press Q`
  (params (Character :type "Character Object Reference") (Roation :type "Rotator Structure") (Transform :type "Transform Structure"))
  (returns (Result :type Boolean))
  (return false))