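; Grappling hook skill component: Q fires a hook projectile with attached cable, using a skill charge, or cancels an active grapple.
; On hit, it lowers gravity, hops the character, attaches the cable to the left hand, then briefly delays opening a Tick gate.
; Tick launches the character toward the hook until a dot product against the impact normal detects overshoot.
; Ending restores gravity, destroys hook and cable, and removes the skill when charges run out.
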(event `self.ReceiveBeginPlay`)

(event `self.ReceiveTick`
  (params (DeltaSeconds :type "Float (single-precision)"))
  (bind _grapple_projectile (`self.Grapple Projectile`))
  (`/Engine/EditorBlueprintResources/StandardMacros.Gate` true :!label _label ; 캐릭터를 훅 방향으로 계속 launch\n그래플 히트되면 열어주고 그래플 끝나면 닫아주기
    (:`Exit`
      (`/Engine/EditorBlueprintResources/StandardMacros.IsValid` _grapple_projectile
        (:`Is Valid`
          (`Character.LaunchCharacter` (`self.Character`) (* (* (`KismetMathLibrary.Normal` (- (`Actor.K2_GetActorLocation` _grapple_projectile) (`Actor.K2_GetActorLocation` (`self.Character`)))) 2000.0) (`GameplayStatics.GetWorldDeltaSeconds`)) false false) ; 훅 방향으로 계속 보냄
          (if (> (`KismetMathLibrary.Dot_VectorVector` (`.ImpactNormal` (`GameplayStatics.BreakHitResult` (`self.Hit Result`))) (`KismetMathLibrary.Normal` (- (`Actor.K2_GetActorLocation` (`self.Grapple Projectile`)) (`Actor.K2_GetActorLocation` (`self.Character`))))) 0.0)
            (`self.End Grappling`) ; 앞쪽범위로 넘어가면 그래플 끊기
          ))))))

(event `OepnGate`
  (goto _label :!via `Open`))

(event `CloseGate`
  (goto _label :!via `Close`))

(fn `Check Can Grapppling`
  (returns (Result :type Boolean))
  (bind _returnvalue (`GameplayStatics.GetPlayerCameraManager` 0))
  (bind _returnvalue_2 (`Actor.GetActorForwardVector` _returnvalue))
  (bind _returnvalue_3 (`PlayerCameraManager.GetCameraLocation` _returnvalue))
  (bind (_outhit _returnvalue_4) (`KismetSystemLibrary.LineTraceSingle` :`Start` (+ _returnvalue_3 (* _returnvalue_2 100.0)) :`End` (+ _returnvalue_3 (* _returnvalue_2 2000.0)) :`TraceChannel` "TraceTypeQuery1" :`DrawDebugType` "ForDuration"))
  (if _returnvalue_4
    (return true)
    (else
      (return false))))

(fn `Client Press Q`
  (params (Character :type "Character Object Reference"))
  (returns (Result :type Boolean))
  (return false))

(fn `Destroy Client Component`
  (returns (Result :type Boolean))
  (return false))

(fn `Destroy Self`
  (returns (Result :type Boolean))
  (`/Game/ShootingGame/GameMode/BP_HyperCharacter.Server Destroy Skill` (`self.Character`)))

(fn `End Grappling`
  (bind _grapple_projectile (`self.Grapple Projectile`))
  (bind _grapple_cable (`self.Grapple Cable`))
  (`self.CloseGate`) ; Tick 끊어서 캐릭터 런치 적용 안되게
  (set `CharacterMovementComponent.GravityScale` (`self.DefaultGravity`) (`Character.CharacterMovement` (`self.Character`)))
  (set `self.Is Grappling Running?` false)
  (`/Engine/EditorBlueprintResources/StandardMacros.IsValid` _grapple_projectile
    (:`Is Valid`
      (`Actor.K2_DestroyActor` _grapple_projectile)
      (`/Engine/EditorBlueprintResources/StandardMacros.IsValid` _grapple_cable
        (:`Is Valid`
          (`Actor.K2_DestroyActor` _grapple_cable)
          (if (<= (`/Game/ShootingGame/GameMode/BP_HyperCharacter.Skill Count` (`self.Character`)) 0)
            (`self.Destroy Self`)))))))

(fn `Event Hit Grappling`
  (params (Hit :type "HitResult Structure"))
  (bind _grapple_cable (`self.Grapple Cable`))
  (set `self.Hit Result` Hit)
  (set `self.Is Grappling Running?` true)
  (set `CharacterMovementComponent.GravityScale` 0.33 (`Character.CharacterMovement` (`self.Character`)))
  (`Character.LaunchCharacter` (`self.Character`) (0.0 0.0 150.0) false true) ; 살짝 위로 점프시키는 용도
  (`/Engine/EditorBlueprintResources/StandardMacros.IsValid` _grapple_cable
    (:`Is Valid`
      (`CableComponent.SetAttachEndToComponent` (`/Game/ShootingGame/Blueprint/Skill/BP_GrappleCable_Test.Cable` _grapple_cable) (`Character.Mesh` (`self.Character`)) "Hand_L") ; 끝을 캐릭터에게 어태치시킴
      (`KismetSystemLibrary.K2_SetTimer` null "Open Gate_Func" 0.2))))

(fn `Event Press E`
  (params (Character :type "Character Object Reference") (True :type Boolean))
  (returns (Result :type Boolean))
  (return false))

(fn `EventPressQ`
  (params (Character :type "Character Object Reference") (Location :type "Vector Structure") (Rotation :type "Rotator Structure") (True :type Boolean))
  (returns (Result :type Boolean))
  (bind _character (`self.Character`))
  (bind _character_2 (`self.Character`))
  (if (`self.Check Grappling Running`)
    (`self.End Grappling`)
    (elif (> (`/Game/ShootingGame/GameMode/BP_HyperCharacter.Skill Count` (`self.Character`)) 0)
      (`/Game/ShootingGame/GameMode/BP_HyperCharacter.Play Sound At Owner` _character "/Game/ShootingGame/Sound/Hook.Hook" 0.0 1.0 (`/Game/ShootingGame/GameMode/BP_HyperCharacter.Skill Sound` _character))
      (bind _returnvalue (`|SpawnActorFromClass` "/Game/ShootingGame/Blueprint/Skill/BP_GrappleProjectile.BP_GrappleProjectile_C" (`KismetMathLibrary.MakeTransform` Location Rotation) "Undefined" "OverrideRootScale" null (`self.Character`) null null)) ; 훅 발사
      (bind _output_get (set `self.Grapple Projectile` _returnvalue))
      (add `/Game/ShootingGame/Blueprint/Skill/BP_GrappleProjectile.GrappleHit` _output_get (`|CreateDelegate` :!event `Event Hit Grappling`)) ; 생성한 훅이 Hit 했을 때 호출되는 바인딩 이벤트
      (bind _returnvalue_2 (`|SpawnActorFromClass` "/Game/ShootingGame/Blueprint/Skill/BP_GrappleCable_Test.BP_GrappleCable_Test_C" (`KismetMathLibrary.MakeTransform` Location Rotation) "Undefined" "OverrideRootScale" null null (`local.Character`)))
      (bind _output_get_2 (set `self.Grapple Cable` _returnvalue_2))
      (`Actor.K2_AttachToActor` _output_get_2 (`self.Grapple Projectile`) "None" "SnapToTarget" "SnapToTarget" "KeepWorld" true) ; 케이블 시작점을 훅에 어태치 시킴.
      (`self.CheckMyPlayer` _character_2
        (:`True`
          (`/Game/ShootingGame/GameMode/BP_HyperCharacter.Server Minus Skill Count` _character_2))))))

(fn `FindLocation`
  (params (Transform :type "Transform Structure"))
  (returns (Result :type Boolean))
  (return false))

(fn `Initialize`
  (params (Chracter :type "Character Object Reference") (`Skill Count` :type Integer))
  (returns (Result :type Boolean))
  (bind _asbp_hyper_character (cast `/Game/ShootingGame/GameMode/BP_HyperCharacter` Chracter))
  (bind _output_get (set `self.Character` _asbp_hyper_character))
  (set `self.DefaultGravity` (`CharacterMovementComponent.GravityScale` (`Character.CharacterMovement` _output_get)))
  (`/Game/ShootingGame/GameMode/BP_HyperCharacter.Update Skill Count Multi` (`self.Character`))
  (return false))

(fn `Open Gate_Func`
  (`self.OepnGate`))

(fn `Push Character`
  (bind _grapple_projectile (`self.Grapple Projectile`))
  (`/Engine/EditorBlueprintResources/StandardMacros.IsValid` _grapple_projectile
    (:`Is Valid`
      (`Character.LaunchCharacter` (`self.Character`) (* (* (`KismetMathLibrary.Normal` (- (`Actor.K2_GetActorLocation` _grapple_projectile) (`Actor.K2_GetActorLocation` (`self.Character`)))) 2000.0) (`GameplayStatics.GetWorldDeltaSeconds`)) false false) ; 훅 방향으로 계속 보냄
      (if (> (`KismetMathLibrary.Dot_VectorVector` (`.ImpactNormal` (`GameplayStatics.BreakHitResult` (`self.Hit Result`))) (`KismetMathLibrary.Normal` (- (`Actor.K2_GetActorLocation` (`self.Grapple Projectile`)) (`Actor.K2_GetActorLocation` (`self.Character`))))) 0.0)
        (`self.End Grappling`) ; 앞쪽범위로 넘어가면 그래플 끊기
      ))))

(fn `Server Press Q`
  (params (Character :type "Character Object Reference"))
  (returns (Result :type Boolean))
  (return false))