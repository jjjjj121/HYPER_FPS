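; Timed buff-skill actor that drains a character's temporary BuffHP back down while a heartbeat effect plays.
; On BeginPlay it starts the heartbeat on HyperCharacter, runs a looping one-second SetOriginalHp timer and limits its lifespan to about ten seconds.
; Each tick subtracts MinusHP from BuffHP on BP_ShootingPlayerState, clearing the timer once none remains.
; Destruction stops the heartbeat.
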(event `self.ReceiveBeginPlay`
  (`/Game/ShootingGame/GameMode/BP_HyperCharacter.Play HeartBeat` (`self.HyperCharacter`))
  (`KismetSystemLibrary.K2_SetTimer` null "SetOriginalHp" 1.0 true)
  (`self.SetLifeSpan` 10.1))

(event `self.ReceiveDestroyed`
  (`/Game/ShootingGame/GameMode/BP_HyperCharacter.Stop HeartBeat` (`self.HyperCharacter`)))

(fn `SetOriginalHp`
  (bind _asbp_shooting_player_state (cast `/Game/ShootingGame/GameMode/BP_ShootingPlayerState` (`Pawn.PlayerState` (`self.HyperCharacter`))))
  (bind _buff_hp (`/Game/ShootingGame/GameMode/BP_ShootingPlayerState.Buff HP` _asbp_shooting_player_state))
  (if (> _buff_hp 0.0)
    (set `/Game/ShootingGame/GameMode/BP_ShootingPlayerState.Buff HP` (- _buff_hp (`self.Minus HP`)) _asbp_shooting_player_state)
    (`KismetSystemLibrary.PrintString` (`KismetStringLibrary.Conv_DoubleToString` (`/Game/ShootingGame/GameMode/BP_ShootingPlayerState.Result HP` _asbp_shooting_player_state)) false false (struct :`R` 0.93948 :`B` 1.0 :`A` 1.0) 3.0)
    (else
      (`KismetSystemLibrary.K2_ClearTimer` null "SetOriginalHp"))))

(fn `UserConstructionScript`)