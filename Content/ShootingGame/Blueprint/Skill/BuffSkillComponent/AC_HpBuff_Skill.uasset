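; HP buff skill component that lets a BP_HyperCharacter drop a buff actor at its feet with Q.
; Initialize caches the character and its player state and refreshes the skill count display.
; EventPressQ spawns an enlarged, team-tagged BP_Skill_HpBuff, decrements the count, and has the character destroy the skill when none remain.
; ClientPressQ and SetOriginalHp subtract BuffHp from ResultHP; the reset timer is unreachable and E does nothing.
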(event `self.ReceiveBeginPlay`)

(event `self.ReceiveTick`
  (params (DeltaSeconds :type "Float (single-precision)")))

(fn `Client Press Q`
  (params (Character :type "Character Object Reference"))
  (returns (Result :type Boolean))
  (bind _player_state (`self.Player State`))
  (bind _output_get (set `/Game/ShootingGame/GameMode/BP_ShootingPlayerState.Result HP` (- (`/Game/ShootingGame/GameMode/BP_ShootingPlayerState.Result HP` _player_state) (`self.Buff Hp`)) _player_state))
  (`KismetSystemLibrary.PrintString` (`KismetStringLibrary.Conv_DoubleToString` _output_get) false false (struct :`R` 1.0 :`G` 0.103262 :`A` 1.0) 30.0))

(fn `Destroy Client Component`
  (returns (Result :type Boolean))
  (return false))

(fn `Destroy Self`
  (returns (Result :type Boolean))
  (`/Game/ShootingGame/GameMode/BP_HyperCharacter.Server Destroy Skill` (`self.Hyper Character`)))

(fn `Event Press E`
  (params (Character :type "Character Object Reference") (True :type Boolean))
  (returns (Result :type Boolean))
  (return false))

(fn `EventPressQ`
  (params (Character :type "Character Object Reference") (Location :type "Vector Structure") (Rotation :type "Rotator Structure") (True :type Boolean))
  (returns (Result :type Boolean))
  (bind _hyper_character (`self.Hyper Character`))
  (if (> (`/Game/ShootingGame/GameMode/BP_HyperCharacter.Skill Count` (`self.Hyper Character`)) 0)
    (`|SpawnActorFromClass` "/Game/ShootingGame/Blueprint/Skill/BuffSkillComponent/BP_Skill_HpBuff.BP_Skill_HpBuff_C" (`KismetMathLibrary.MakeTransform` (`KismetMathLibrary.MakeVector` (.x (.location (`Actor.GetTransform` (`Controller.K2_GetPawn` (`Pawn.GetController` (`self.Hyper Character`)))))) (.y (.location (`Actor.GetTransform` (`Controller.K2_GetPawn` (`Pawn.GetController` (`self.Hyper Character`)))))) (+ (.z (.location (`Actor.GetTransform` (`Controller.K2_GetPawn` (`Pawn.GetController` (`self.Hyper Character`)))))) -50.0)) (struct) (* (.scale (`Actor.GetTransform` (`Controller.K2_GetPawn` (`Pawn.GetController` (`self.Hyper Character`))))) 10.0)) "Undefined" "OverrideRootScale" null _hyper_character (`/Game/ShootingGame/GameMode/BP_HyperCharacter.Team` _hyper_character) null)
    (`/Game/ShootingGame/GameMode/BP_HyperCharacter.Server Minus Skill Count` (`self.Hyper Character`))
    (if (<= (`/Game/ShootingGame/GameMode/BP_HyperCharacter.Skill Count` (`self.Hyper Character`)) 0)
      (`self.Destroy Self`))))

(fn `FindLocation`
  (params (Transform :type "Transform Structure"))
  (returns (Result :type Boolean))
  (return false))

(fn `Get Value`
  (returns (Ratation :type "Rotator Structure") (Transform :type "Transform Structure"))
  (return))

(fn `Initialize`
  (params (Chracter :type "Character Object Reference") (`Skill Count` :type Integer))
  (returns (Result :type Boolean))
  (bind _asbp_hyper_character (cast `/Game/ShootingGame/GameMode/BP_HyperCharacter` Chracter))
  (bind _output_get (set `self.Hyper Character` _asbp_hyper_character))
  (bind _asbp_shooting_player_state (cast `/Game/ShootingGame/GameMode/BP_ShootingPlayerState` (`Pawn.PlayerState` _output_get)))
  (set `self.Player State` _asbp_shooting_player_state)
  (`/Game/ShootingGame/GameMode/BP_HyperCharacter.Update Skill Count Multi` (`self.Hyper Character`)))

(fn `Server Press Q`
  (params (Character :type "Character Object Reference") (Roation :type "Rotator Structure") (Transform :type "Transform Structure"))
  (returns (Result :type Boolean))
  (`|SpawnActorFromClass` "/Game/ShootingGame/Blueprint/Skill/BuffSkillComponent/BP_Skill_HpBuff.BP_Skill_HpBuff_C" (`KismetMathLibrary.MakeTransform` (`KismetMathLibrary.MakeVector` (.x (.location (`Actor.GetTransform` (`Controller.K2_GetPawn` (`Pawn.GetController` (`self.Hyper Character`)))))) (.y (.location (`Actor.GetTransform` (`Controller.K2_GetPawn` (`Pawn.GetController` (`self.Hyper Character`)))))) (+ (.z (.location (`Actor.GetTransform` (`Controller.K2_GetPawn` (`Pawn.GetController` (`self.Hyper Character`)))))) -50.0)) (struct) (* (.scale (`Actor.GetTransform` (`Controller.K2_GetPawn` (`Pawn.GetController` (`self.Hyper Character`))))) 10.0)) "Undefined" "OverrideRootScale" null (`self.Hyper Character`) "NewEnumerator0" null))

(fn `SetOriginalHp`
  (bind _player_state (`self.Player State`))
  (bind _output_get (set `/Game/ShootingGame/GameMode/BP_ShootingPlayerState.Result HP` (- (`/Game/ShootingGame/GameMode/BP_ShootingPlayerState.Result HP` _player_state) (`self.Buff Hp`)) _player_state))
  (`KismetSystemLibrary.PrintString` (`KismetStringLibrary.Conv_DoubleToString` _output_get) false false (struct :`R` 1.0 :`G` 0.103262 :`A` 1.0) 30.0))