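; Skill spawner actor that scatters random skill actors over the navigable area around itself at BeginPlay.
; A delay-loop macro waits briefly, then calls Spawn Actor repeatedly in one burst.
; On authority, Spawn Actor picks a random navmesh point, traces down to WorldStatic and spawns just above the hit, recursively retrying on a miss.
; Timer-based respawn functions exist, but nothing here binds them.
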(event `self.ReceiveBeginPlay`
  (`self.Delay For loop` 1 15 0.6
    (:`Loop Body`
      (`self.Spawn Actor`))))

(fn `Destroy Skill`
  (params (DestroyedActor :type "Actor Object Reference"))
  (`KismetSystemLibrary.K2_SetTimer` null "Random Spawn" (`KismetMathLibrary.Conv_IntToDouble` (`KismetMathLibrary.RandomIntegerInRange` 20 30))))

(fn `Random Spawn`
  (`KismetSystemLibrary.K2_SetTimer` null "Spawn Actor" (`KismetMathLibrary.Conv_IntToDouble` (`KismetMathLibrary.RandomIntegerInRange` 1 5))))

(fn `Spawn Actor`
  (bind (_returnvalue_location _returnvalue_rotation _returnvalue_scale) (`KismetMathLibrary.BreakTransform` (`self.GetTransform`)))
  (bind (_returnvalue_x _returnvalue_y _returnvalue_z) (`KismetMathLibrary.BreakVector` (`self.K2_GetActorLocation`)))
  (`/Engine/EditorBlueprintResources/ActorMacros.Switch Has Authority`
    (:`Authority`
      (bind _randomlocation (`NavigationSystemV1.K2_GetRandomLocationInNavigableRadius` (`KismetMathLibrary.MakeVector` _returnvalue_x _returnvalue_y _returnvalue_z) 7000.0 null null))
      (bind (_outhit _returnvalue) (`KismetSystemLibrary.LineTraceSingleForObjects` :`Start` _randomlocation :`End` (`KismetMathLibrary.MakeVector` (.x _randomlocation) (.y _randomlocation) -100000.0) :`ObjectTypes` (`|MakeArray` "ObjectTypeQuery1" :!type "EObjectTypeQuery Enum") :`DrawDebugType` "ForDuration"))
      (if _returnvalue
        (bind _returnvalue_2 (`|SpawnActorFromClass` (`KismetArrayLibrary.Array_Random` (`self.Skill`)) (`KismetMathLibrary.MakeTransform` (`KismetMathLibrary.MakeVector` (.x (`.Location` (`GameplayStatics.BreakHitResult` _outhit))) (.y (`.Location` (`GameplayStatics.BreakHitResult` _outhit))) (+ (.z (`.Location` (`GameplayStatics.BreakHitResult` _outhit))) 100.0)) _returnvalue_rotation _returnvalue_scale) "AdjustIfPossibleButAlwaysSpawn" "OverrideRootScale" null 3 self null))
        (set `self.Spawn Skill` _returnvalue_2)
        (else
          (`self.Spawn Actor`))))))

(fn `UserConstructionScript`)