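; Armor pickup for the shooting game that flies to the character who claims it and applies its armor values.
; A press locks in the owning character and starts a looping timer that hides the wisp and homes toward them with growing speed.
; Overlapping that character overwrites Armor and MaxArmor on their player state, then destroys the pickup.
; On destruction it notifies the game mode to check armor spawning for its spawner.
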(event `self.ReceiveBeginPlay`
  (bind _asbp_hyper_fpsgame_mode (cast `/Game/ShootingGame/GameMode/MultiPlay/BP_HyperFPSGameMode` (`GameplayStatics.GetGameMode`)))
  (set `self.Game Mode` _asbp_hyper_fpsgame_mode))

(event `self.Core.OnComponentBeginOverlap`
  (params (OverlappedComponent :type "PrimitiveComponent Object Reference") (OtherActor :type "Actor Object Reference") (OtherComp :type "PrimitiveComponent Object Reference") (OtherBodyIndex :type Integer) (bFromSweep :type Boolean) (SweepResult :type "HitResult Structure (by ref)"))
  (if (`self.Is Press?`)
    (if (== OtherActor (`self.Own Character`))
      (bind _asbp_shooting_player_state (cast `/Game/ShootingGame/GameMode/BP_ShootingPlayerState` (`Pawn.PlayerState` (`self.Own Character`))))
      (set `/Game/ShootingGame/GameMode/BP_ShootingPlayerState.Max Armor` (`self.Default Armor`) _asbp_shooting_player_state)
      (set `/Game/ShootingGame/GameMode/BP_ShootingPlayerState.Armor` (`self.Cur Armor`) _asbp_shooting_player_state)
      (`self.K2_DestroyActor`))))

(event `self.ReceiveDestroyed`
  (`/Game/ShootingGame/GameMode/MultiPlay/BP_HyperFPSGameMode.Check Spawn Armor` (`self.Game Mode`) (`self.Own Spawner`)))

(fn `Check Cur Info`
  (returns (`Cur Data` :type Integer) (`Default Data` :type Integer))
  (return (`KismetMathLibrary.FTrunc` (`self.Cur Armor`)) (`KismetMathLibrary.FTrunc` (`self.Default Armor`))))

(fn `EventCanPickUp`
  (returns (`Can Pick UP?` :type Boolean))
  (return (not (`KismetSystemLibrary.IsValid` (`self.Own Character`)))))

(fn `EventPress`
  (params (Character :type "Character Object Reference"))
  (returns (Result :type Boolean))
  (bind _asbp_hyper_character (cast `/Game/ShootingGame/GameMode/BP_HyperCharacter` Character))
  (set `self.Own Character` _asbp_hyper_character)
  (set `self.Is Press?` true)
  (`KismetSystemLibrary.K2_SetTimer` null "Move Character" 0.01 true))

(fn `EventRelease`
  (params (Character :type "Character Object Reference"))
  (returns (Result :type Boolean))
  (return false))

(fn `Move Character`
  (set `self.Delta Value` (+ (`self.Delta Value`) 10.0))
  (`SceneComponent.SetVisibility` (`self.P_Wisp`) false false)
  (`self.K2_SetActorRotation` (`KismetMathLibrary.FindLookAtRotation` (`self.K2_GetActorLocation`) (`self.K2_GetActorLocation` (`self.Own Character`))))
  (`self.K2_AddActorWorldOffset` (* (`self.GetActorForwardVector`) (* (`GameplayStatics.GetWorldDeltaSeconds`) (`self.Delta Value`)))))

(fn `UserConstructionScript`)