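; Armor spawner actor that scatters random armor pickups across the navigable area around it, spawning a batch at BeginPlay after a short delay.
; On authority, it picks a navigable point, traces down to world-static ground, retrying on a miss, then spawns a random T_Armor row's actor with itself as owner spawner.
; DestroyArmor sets a randomized timer for "Spawn Random", which matches no function here; RandomSpawn separately schedules a delayed spawn.
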(event `self.ReceiveBeginPlay`
  (`self.Delay For loop` 1 5 0.6
    (:`Loop Body`
      (`self.Spawn Armor Func`))))

(fn `Destroy Armor`
  (params (DestroyedActor :type "Actor Object Reference"))
  (`KismetSystemLibrary.K2_SetTimer` null "Spawn Random" (`KismetMathLibrary.Conv_IntToDouble` (`KismetMathLibrary.RandomIntegerInRange` 20 30))))

(fn `Get Random Armor Name`
  (returns (WeaponName :type "Name (by ref)"))
  (bind _outrownames (`DataTableFunctionLibrary.GetDataTableRowNames` "/Game/ShootingGame/Data/T_Armor.T_Armor"))
  (return (`|GetArrayItem` _outrownames (`KismetMathLibrary.RandomInteger` (`KismetArrayLibrary.Array_Length` _outrownames)))))

(fn `Random Spawn`
  (`KismetSystemLibrary.K2_SetTimer` null "Spawn Armor Func" (`KismetMathLibrary.Conv_IntToDouble` (`KismetMathLibrary.RandomIntegerInRange` 10 20))))

(fn `Spawn Armor Func`
  (bind (_returnvalue_location _returnvalue_rotation _returnvalue_scale) (`KismetMathLibrary.BreakTransform` (`self.GetTransform`)))
  (bind (_returnvalue_x _returnvalue_y _returnvalue_z) (`KismetMathLibrary.BreakVector` (`self.K2_GetActorLocation`)))
  (`/Engine/EditorBlueprintResources/ActorMacros.Switch Has Authority`
    (:`Authority`
      (bind _randomlocation (`NavigationSystemV1.K2_GetRandomLocationInNavigableRadius` (`KismetMathLibrary.MakeVector` _returnvalue_x _returnvalue_y _returnvalue_z) 7000.0 null null))
      (bind (_outhit _returnvalue) (`KismetSystemLibrary.LineTraceSingleForObjects` :`Start` _randomlocation :`End` (`KismetMathLibrary.MakeVector` (.x _randomlocation) (.y _randomlocation) -100000.0) :`ObjectTypes` (`|MakeArray` "ObjectTypeQuery1" :!type "EObjectTypeQuery Enum") :`DrawDebugType` "ForDuration"))
      (if _returnvalue
        (bind _returnvalue_2 (`|GetDataTableRow` "/Game/ShootingGame/Data/T_Armor.T_Armor" (`self.Get Random Armor Name`))
          (:`then`
            (bind (_armoractor _defaultarmor) (break `/Game/ShootingGame/Data/ST_Armor` _returnvalue_2))
            (bind _returnvalue_3 (`|SpawnActorFromClass` _armoractor (`KismetMathLibrary.MakeTransform` (`KismetMathLibrary.MakeVector` (.x (`.Location` (`GameplayStatics.BreakHitResult` _outhit))) (.y (`.Location` (`GameplayStatics.BreakHitResult` _outhit))) (+ (.z (`.Location` (`GameplayStatics.BreakHitResult` _outhit))) 100.0)) _returnvalue_rotation _returnvalue_scale) "AdjustIfPossibleButAlwaysSpawn" "OverrideRootScale" null _defaultarmor null _defaultarmor self null))
            (set `self.Spawn Armor` _returnvalue_3)))
        (else
          (`self.Spawn Armor Func`))))))

(fn `UserConstructionScript`)