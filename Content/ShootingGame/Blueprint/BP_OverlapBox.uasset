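; BP_OverlapBox is a one-shot pickup box in the shooting game that spawns a BP_Weapon at its location when something overlaps its Cube.
; The overlap is handled only with authority, so the server hides the Cube, disables its collision and spawns the weapon.
; It then calls ResBeginOverlap, which repeats the hide and collision disable.
; A character-controller ownership fragment is left unconnected and never runs.
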(event `self.Cube.OnComponentBeginOverlap`
  (params (OverlappedComponent :type "PrimitiveComponent Object Reference") (OtherActor :type "Actor Object Reference") (OtherComp :type "PrimitiveComponent Object Reference") (OtherBodyIndex :type Integer) (bFromSweep :type Boolean) (SweepResult :type "HitResult Structure (by ref)"))
  (bind _cube (`self.Cube`))
  (`/Engine/EditorBlueprintResources/ActorMacros.Switch Has Authority` ; 서버만 나가게 제한걸어서\n오버랩 유무를 서버에서만 판단하게함
    (:`Authority`
      (`SceneComponent.SetVisibility` _cube false false)
      (`PrimitiveComponent.SetCollisionEnabled` _cube "NoCollision")
      (`|SpawnActorFromClass` "/Game/ShootingGame/Blueprint/Weapon/BP_Weapon.BP_Weapon_C" (`KismetMathLibrary.MakeTransform` (`self.K2_GetActorLocation`)) "Undefined" "OverrideRootScale" null (struct) null)
      (`self.ResBeginOverlap`))))

(event `self.ReceiveBeginPlay`)

(event `ResBeginOverlap`
  (bind _cube (`self.Cube`))
  (`SceneComponent.SetVisibility` _cube false false)
  (`PrimitiveComponent.SetCollisionEnabled` _cube "NoCollision"))

(fn `UserConstructionScript`)